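; BP_Loadout is an interactable that opens the loadout menu for the player.
; On BeginPlay it casts the first player character to BP_Player and stores it.
; Its Loadout and Menu interaction functions fire OpenMenu, which has the player open WBP_Loadout_Main without pausing the game.
; The CommandDeck and MissionSelect interaction functions do nothing, and all four return false.
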(event `self.ReceiveBeginPlay`
  (bind _asbp_player (cast `/Game/Blueprints/Player/BP_Player` (`GameplayStatics.GetPlayerCharacter` 0)))
  (set `self.As BP Player` _asbp_player))

(event `OpenMenu`
  (`/Game/Blueprints/Player/BP_Player.OpenMenu` (`self.As BP Player`) "/Game/Widgets/Loadout/WBP_Loadout_Main.WBP_Loadout_Main_C" false))

(fn `Interact_CommandDeck`
  (params (Interactor :type "/Game/Blueprints/Player/BP_Player Object Reference"))
  (returns (`Success?` :type Boolean))
  (return false))

(fn `Interact_Loadout`
  (params (Interactor :type "/Game/Blueprints/Player/BP_Player Object Reference"))
  (returns (`Success?` :type Boolean))
  (`self.OpenMenu`)
  (return false))

(fn `Interact_Menu`
  (params (Interactor :type "/Game/Blueprints/Player/BP_Player Object Reference"))
  (returns (`Success?` :type Boolean))
  (`self.OpenMenu`)
  (return false))

(fn `Interact_MissionSelect`
  (params (Interactor :type "/Game/Blueprints/Player/BP_Player Object Reference"))
  (returns (`Success?` :type Boolean))
  (return false))

(fn `UserConstructionScript`)