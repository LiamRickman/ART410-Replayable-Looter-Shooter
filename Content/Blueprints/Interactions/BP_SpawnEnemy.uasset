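; BP_SpawnEnemy is an interactable spawner that creates a Standard or Sniper enemy, with a text render showing the selected type.
; Its InteractMenu function calls SpawnEnemy, which picks the enemy class from the EnemyToSpawn setting.
; The enemy appears at a random point within the bounds of the BP_SpawnEnemy_Area actor found in the level, raised slightly on Z.
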(event `SpawnEnemy`
  (switch `string` (`KismetTextLibrary.Conv_TextToString` (`self.EnemyToSpawn`))
    (:`Standard`
      (set `self.EnemyClass` "/Game/Blueprints/Enemies/Standard/BP_Enemy_Standard.BP_Enemy_Standard_C"))
    (:`Sniper`
      (set `self.EnemyClass` "/Game/Blueprints/Enemies/Sniper/BP_Enemy_Sniper.BP_Enemy_Sniper_C")))
  (bind _returnvalue (`GameplayStatics.GetActorOfClass` "/Game/Blueprints/Interactions/BP_SpawnEnemy_Area.BP_SpawnEnemy_Area_C"))
  (bind (_origin _boxextent) (`self.GetActorBounds` _returnvalue false false))
  (`|SpawnActorFromClass` (`self.EnemyClass`) (`KismetMathLibrary.MakeTransform` (+ (`KismetMathLibrary.RandomPointInBoundingBox` _origin _boxextent) (0.0 0.0 100.0))) "Undefined" "OverrideRootScale" null null))

(event `self.ReceiveBeginPlay`
  (`TextRenderComponent.K2_SetText` (`self.TextRender`) (`self.EnemyToSpawn`)))

(fn `Interact_Menu`
  (params (Interactor :type "/Game/Blueprints/Player/BP_Player Object Reference"))
  (returns (`Success?` :type Boolean))
  (`self.SpawnEnemy`)
  (return false))

(fn `UserConstructionScript`)