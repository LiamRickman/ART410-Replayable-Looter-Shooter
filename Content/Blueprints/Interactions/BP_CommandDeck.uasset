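; BP_CommandDeck is an interactable command deck that opens the player's command deck menu and can spawn enemies in a linked area.
; Interacting passes the deck to BP_Player's menu toggle, and a text render shows its identifier from BeginPlay.
; SpawnEnemies, not called within this graph, places configured counts of standard and sniper enemies at random, raised points inside EnemySpawnArea's bounds.
; Loadout and mission select interactions are stubs.
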(event `OpenCommandDeckUI`
  (bind _asbp_player (cast `/Game/Blueprints/Player/BP_Player` (`GameplayStatics.GetPlayerCharacter` 0)))
  (`/Game/Blueprints/Player/BP_Player.ToggleCommandDeckMenu` _asbp_player self))

(event `self.ReceiveBeginPlay`
  (`TextRenderComponent.K2_SetText` (`self.TextRender`) (`self.TextIdentifier`)))

(event `SpawnEnemies`
  (bind (_enemiestospawn_standard _enemiestospawn_sniper) (break `/Game/Blueprints/Interactions/STR_EnemyCount` (`self.EnemiesToSpawn`)))
  (bind _enemiestospawn_standard_2 (break `/Game/Blueprints/Interactions/STR_EnemyCount` (`self.EnemiesToSpawn`)))
  (bind (_origin _boxextent) (`self.GetActorBounds` (`self.EnemySpawnArea`) false false))
  (bind (_origin_2 _boxextent_2) (`self.GetActorBounds` (`self.EnemySpawnArea`) false false))
  (for _ (range 1 (+ _enemiestospawn_standard_2 1))
    (`|SpawnActorFromClass` "/Game/Blueprints/Enemies/Standard/BP_Enemy_Standard.BP_Enemy_Standard_C" (`KismetMathLibrary.MakeTransform` (+ (`KismetMathLibrary.RandomPointInBoundingBox` _origin _boxextent) (0.0 0.0 100.0))) "Undefined" "OverrideRootScale" null null))
  (for _ (range 1 (+ _enemiestospawn_sniper 1))
    (`|SpawnActorFromClass` "/Game/Blueprints/Enemies/Sniper/BP_Enemy_Sniper.BP_Enemy_Sniper_C" (`KismetMathLibrary.MakeTransform` (+ (`KismetMathLibrary.RandomPointInBoundingBox` _origin_2 _boxextent_2) (0.0 0.0 100.0))) "Undefined" "OverrideRootScale" null null)))

(fn `Interact_CommandDeck`
  (params (Interactor :type "/Game/Blueprints/Player/BP_Player Object Reference"))
  (returns (`Success?` :type Boolean))
  (`self.OpenCommandDeckUI`)
  (return false))

(fn `Interact_Loadout`
  (params (Interactor :type "/Game/Blueprints/Player/BP_Player Object Reference"))
  (returns (`Success?` :type Boolean)))

(fn `Interact_MissionSelect`
  (params (Interactor :type "/Game/Blueprints/Player/BP_Player Object Reference"))
  (returns (`Success?` :type Boolean))
  (return false))

(fn `UserConstructionScript`)