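; First-person player character Blueprint with movement, sprint, crouch, jump, shooting, reload, aim-down-sights and rifle/revolver switching.
; Held fire loops on a Delay, spending ammo, drawing debug line traces from the weapon socket and adding random recoil; hits apply nothing.
; Delay loops ramp the ADS alpha, Tick drives curve-based sway, and a timeline changes sprint FOV.
; BeginPlay creates the HUD, caches the AnimBP and fills ammo.
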(event `InputAction|Shoot/Fire`
  (params (Key :type "Key Structure"))
  (bind _weapon (`self.Weapon`))
  (bind _returnvalue (`SceneComponent.GetSocketLocation` _weapon "AimSocket"))
  ;[1 1 1] FireWeapon
  (:`Pressed`
    (set `self.FireButtonPressed` true)
    (if (`self.IsReloading`) :!label _label
      _
      (elif (> (`self.CurrentAmmo`) 0)
        (`KismetSystemLibrary.LineTraceSingle` :`Start` _returnvalue :`End` (+ _returnvalue (* (`KismetMathLibrary.GetForwardVector` (`SceneComponent.GetSocketRotation` _weapon "AimSocket")) 100000)) :`TraceChannel` "TraceTypeQuery1" :`DrawDebugType` "ForDuration" :`DrawTime` 1.0)
        ;;[1 1 1] Vertical Recoil
        (if (< (`self.BulletsShot`) 31)
          (`self.AddControllerPitchInput` (`KismetMathLibrary.RandomFloatInRange` -0.1 -0.2)))
        ;;[1 1 1] Horizontal Recoil
        (`self.AddControllerYawInput` (`KismetMathLibrary.RandomFloatInRange` -0.25 0.25))
        (`/Engine/EditorBlueprintResources/StandardMacros.IncrementInt` (`self.BulletsShot`)
          (:`  `
            (`/Engine/EditorBlueprintResources/StandardMacros.DecrementInt` (`self.CurrentAmmo`)
              (:`  `
                (`KismetSystemLibrary.Delay` 0.05)
                (if (`self.FireButtonPressed`)
                  (goto _label)))))))))
  (:`Released`
    (set `self.FireButtonPressed` false)
    (set `self.BulletsShot` 0)))

(event `self.ReceiveBeginPlay`
  (`KismetSystemLibrary.Delay` 0.1)
  (set `self.PlayerController` (`GameplayStatics.GetPlayerController` 0))
  (`self.ShowInGameHUD`)
  (bind _asabp_player (cast `/Game/Animations/Player/ABP_Player` (`SkeletalMeshComponent.GetAnimInstance` (`self.FirstPersonMesh`))))
  (set `self.AnimInstance` _asabp_player)
  (set `self.CurrentAmmo` (`self.MaxAmmo`)))

(event `self.ReceiveTick`
  (params (DeltaSeconds :type "Float (single-precision)"))
  (if (`self.IsAimButtonPressed`)
    (set `self.WeaponSwayVector` (`KismetMathLibrary.VInterpTo` (`self.WeaponSwayVector`) (0.0 0.0 0.0) DeltaSeconds 10.0))
    (else
      (set `self.WeaponSwayVector` (`CurveVector.GetVectorValue` (`self.RifleSwayCurve`) (`KismetSystemLibrary.GetGameTimeInSeconds`))))))

(event `InputAction|Interact`
  (params (Key :type "Key Structure"))
  ;[1 1 1] Raise/Lower
  (:`Pressed`
    (`|PlayMontage` (`self.FirstPersonMesh`) "/Game/Animations/Player/AssaultRifle/AM_AssaultRifle_Lower.AM_AssaultRifle_Lower"
      (:`OnBlendOut`
        (`|PlayMontage` (`self.FirstPersonMesh`) "/Game/Animations/Player/AssaultRifle/AM_AssaultRifle_Raise.AM_AssaultRifle_Raise")))))

(event `InputAction|Reload`
  (params (Key :type "Key Structure"))
  ;[1 1 1] Reload
  (:`Pressed`
    (if (not (`self.IsReloading`))
      (set `self.IsReloading` true)
      (`|PlayMontage` (`self.FirstPersonMesh`) "/Game/Animations/Player/AssaultRifle/AM_AssaultRifle_Reload.AM_AssaultRifle_Reload"
        (:`then`
          (`SkeletalMeshComponent.PlayAnimation` (`self.Weapon`) "/Game/Animations/Weapons/AssaultRifle/AS_AssaultRifle_Reload_Gun.AS_AssaultRifle_Reload_Gun" false))
        (:`OnCompleted`
          (set `self.IsReloading` false)
          (set `self.CurrentAmmo` (`self.MaxAmmo`)))))))

(event `InputAxis|Forward/Back`
  (params (AxisValue :type "Float (single-precision)"))
  (bind (_returnvalue_roll _returnvalue_pitch _returnvalue_yaw) (`KismetMathLibrary.BreakRotator` (`self.GetControlRotation`)))
  ;[1 1 1] Movement Controls
  (bind _output_get (set `self.BS_MoveFwd` AxisValue))
  (`self.AddMovementInput` (`KismetMathLibrary.GetForwardVector` (`KismetMathLibrary.MakeRotator` 0.0 0.0 _returnvalue_yaw)) _output_get))

(event `InputAxis|Left/Right`
  (params (AxisValue :type "Float (single-precision)"))
  (bind (_returnvalue_roll _returnvalue_pitch _returnvalue_yaw) (`KismetMathLibrary.BreakRotator` (`self.GetControlRotation`)))
  ;[1 1 1] Movement Controls
  (bind _output_get (set `self.BS_MoveRight` AxisValue))
  (`self.AddMovementInput` (`KismetMathLibrary.GetRightVector` (`KismetMathLibrary.MakeRotator` 0.0 0.0 _returnvalue_yaw)) _output_get))

(event `InputAxis|LookUp/Down`
  (params (AxisValue :type "Float (single-precision)"))
  ;[1 1 1] Mouse Controls
  (bind _output_get (set `self.BS_LookUp` (* AxisValue (`self.MouseSens`))))
  (`self.AddControllerPitchInput` _output_get))

(event `InputAction|ADS`
  (params (Key :type "Key Structure"))
  ;[1 1 1] ADS
  (:`Pressed`
    (set `self.IsAimButtonPressed` true)
    (set `self.AimAlpha` (`KismetMathLibrary.FClamp` (+ (`self.AimAlpha`) 0.15)) :!label _label_2)
    (`KismetSystemLibrary.Delay` 0.01)
    (if (not (or (not (`self.IsAimButtonPressed`)) (>= (`self.AimAlpha`) 1.0)))
      (goto _label_2)))
  (:`Released`
    (set `self.IsAimButtonPressed` false)
    (set `self.AimAlpha` (`KismetMathLibrary.FClamp` (- (`self.AimAlpha`) 0.15)) :!label _label_3)
    (`KismetSystemLibrary.Delay` 0.01)
    (if (not (or (`self.IsAimButtonPressed`) (<= (`self.AimAlpha`) 0.0)))
      (goto _label_3))))

(event `InputAxis|LookLeft/Right`
  (params (AxisValue :type "Float (single-precision)"))
  ;[1 1 1] Mouse Controls
  (bind _output_get (set `self.BS_LookRight` (* AxisValue (`self.MouseSens`))))
  (`self.AddControllerYawInput` _output_get))

(event `InputAction|Sprint`
  (params (Key :type "Key Structure"))
  (bind _charactermovement (`self.CharacterMovement`))
  ;[1 1 1] Sprint Controls
  (:`Pressed`
    (set `CharacterMovementComponent.MaxWalkSpeed` (`self.SprintSpeed`) _charactermovement)
    (`self.SprintCamera` true))
  (:`Released`
    (set `CharacterMovementComponent.MaxWalkSpeed` (`self.WalkSpeed`) _charactermovement)
    (`self.SprintCamera` false)))

(event `SprintCamera`
  (params (IsRunning :type Boolean))
  ;[1 1 1] Sprint Camera FOV
  (if IsRunning
    (bind (_direction _movecameratrack) (`Timeline|T_MoveCamera` :!label _label_4)
      (:`Update`
        (`CameraComponent.SetFieldOfView` (`self.FirstPersonCamera`) _movecameratrack)))
    (else
      (goto _label_4 :!via `Reverse`))))

(event `InputAction|Crouch`
  (params (Key :type "Key Structure"))
  ;[1 1 1] Crouch Controls
  (:`Pressed`
    (if (`NavMovementComponent.IsMovingOnGround` (`self.CharacterMovement`))
      (`self.Crouch`)
      (else
        (`self.UnCrouch` :!label _label_5))))
  (:`Released`
    (goto _label_5)))

(event `InputAction|Primary`
  (params (Key :type "Key Structure"))
  (:`Pressed`
    (`SkinnedMeshComponent.SetSkinnedAssetAndUpdate` (`self.Weapon`) "/Game/Meshes/Weapons/AssaultRifle/SK_AssaultRifle.SK_AssaultRifle" true)
    (set `self.CurrentWeaponID` 1)))

(event `InputAction|Secondary`
  (params (Key :type "Key Structure"))
  (:`Pressed`
    (`SkinnedMeshComponent.SetSkinnedAssetAndUpdate` (`self.Weapon`) "/Game/Meshes/Weapons/Revolver/SK_Revolver.SK_Revolver" true)
    (set `self.CurrentWeaponID` 2)))

(event `InputAction|Jump`
  (params (Key :type "Key Structure"))
  ;[1 1 1] Jump Controls
  (:`Pressed`
    (if (`NavMovementComponent.IsMovingOnGround` (`self.CharacterMovement`))
      (`self.Jump`))))

(fn `ShowInGameHUD`
  (`/Engine/EditorBlueprintResources/StandardMacros.IsValid` (`self.In-Game HUD`)
    (:`Is Valid`
      _)
    (:`Is Not Valid`
      (bind _returnvalue (`|CreateWidget` "/Game/Widgets/WBP_In-Game_HUD.WBP_In-Game_HUD_C" (`self.PlayerController`)))
      (bind _output_get (set `self.In-Game HUD` _returnvalue))))
  (`UserWidget.AddToViewport` _output_get 0)
  (return))

(fn `UserConstructionScript`)