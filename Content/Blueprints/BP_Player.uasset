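; BP_Player is the first-person player character, handling movement, mouse look, sprint, crouch, jump and rifle actions, and showing the in-game HUD shortly after BeginPlay.
; Axis inputs drive yaw-relative movement and sensitivity-scaled look, storing BS-prefixed values alongside.
; ADS ramps AimAlpha through self-looping Delays, while sprint changes walk speed and plays or reverses a camera FOV timeline.
; Reload and Interact play arm montages, with reload also animating the weapon.
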(event `self.ReceiveBeginPlay`
  (`KismetSystemLibrary.Delay` 0.1)
  (set `self.PlayerController` (`GameplayStatics.GetPlayerController` 0))
  (`self.ShowInGameHUD`))

(event `InputAction|Interact`
  (params (Key :type "Key Structure"))
  (:`Pressed`
    (`|PlayMontage` (`self.FirstPersonMesh`) "/Game/Animations/Player/AM_AssaultRifle_Lower.AM_AssaultRifle_Lower"
      (:`OnBlendOut`
        (`|PlayMontage` (`self.FirstPersonMesh`) "/Game/Animations/Player/AM_AssaultRifle_Raise.AM_AssaultRifle_Raise")))))

(event `InputAxis|Forward/Back`
  (params (AxisValue :type "Float (single-precision)"))
  (bind (_returnvalue_roll _returnvalue_pitch _returnvalue_yaw) (`KismetMathLibrary.BreakRotator` (`self.GetControlRotation`)))
  ;[1 1 1] Movement Controls
  (bind _output_get (set `self.BS_MoveFwd` AxisValue))
  (`self.AddMovementInput` (`KismetMathLibrary.GetForwardVector` (`KismetMathLibrary.MakeRotator` 0.0 0.0 _returnvalue_yaw)) _output_get))

(event `InputAction|Reload`
  (params (Key :type "Key Structure"))
  (:`Pressed`
    (`|PlayMontage` (`self.FirstPersonMesh`) "/Game/Animations/Player/AM_AssaultRifle_Reload.AM_AssaultRifle_Reload"
      (:`then`
        (`SkeletalMeshComponent.PlayAnimation` (`self.Weapon`) "/Game/Animations/Weapons/AssaultRifle/AS_AssaultRifle_Reload_Gun.AS_AssaultRifle_Reload_Gun" false)))))

(event `InputAxis|Left/Right`
  (params (AxisValue :type "Float (single-precision)"))
  (bind (_returnvalue_roll _returnvalue_pitch _returnvalue_yaw) (`KismetMathLibrary.BreakRotator` (`self.GetControlRotation`)))
  ;[1 1 1] Movement Controls
  (bind _output_get (set `self.BS_MoveRight` AxisValue))
  (`self.AddMovementInput` (`KismetMathLibrary.GetRightVector` (`KismetMathLibrary.MakeRotator` 0.0 0.0 _returnvalue_yaw)) _output_get))

(event `InputAction|ADS`
  (params (Key :type "Key Structure"))
  (:`Pressed`
    (set `self.IsAimButtonPressed` true)
    (set `self.AimAlpha` (`KismetMathLibrary.FClamp` (+ (`self.AimAlpha`) 0.15)) :!label _label)
    (`KismetSystemLibrary.Delay` 0.01)
    (if (not (or (not (`self.IsAimButtonPressed`)) (>= (`self.AimAlpha`) 1.0)))
      (goto _label)))
  (:`Released`
    (set `self.IsAimButtonPressed` false)
    (set `self.AimAlpha` (`KismetMathLibrary.FClamp` (- (`self.AimAlpha`) 0.15)) :!label _label_2)
    (`KismetSystemLibrary.Delay` 0.01)
    (if (not (or (`self.IsAimButtonPressed`) (<= (`self.AimAlpha`) 0.0)))
      (goto _label_2))))

(event `InputAxis|LookUp/Down`
  (params (AxisValue :type "Float (single-precision)"))
  ;[1 1 1] Mouse Controls
  (bind _output_get (set `self.BS_LookUp` (* AxisValue (`self.MouseSens`))))
  (`self.AddControllerPitchInput` _output_get))

(event `InputAxis|LookLeft/Right`
  (params (AxisValue :type "Float (single-precision)"))
  ;[1 1 1] Mouse Controls
  (bind _output_get (set `self.BS_LookRight` (* AxisValue (`self.MouseSens`))))
  (`self.AddControllerYawInput` _output_get))

(event `InputAction|Sprint`
  (params (Key :type "Key Structure"))
  (bind _charactermovement (`self.CharacterMovement`))
  ;[1 1 1] Sprint Controls
  (:`Pressed`
    (set `CharacterMovementComponent.MaxWalkSpeed` (`self.SprintSpeed`) _charactermovement)
    (`self.SprintCamera` true))
  (:`Released`
    (set `CharacterMovementComponent.MaxWalkSpeed` (`self.WalkSpeed`) _charactermovement)
    (`self.SprintCamera` false)))

(event `SprintCamera`
  (params (IsRunning :type Boolean))
  ;[1 1 1] Sprint Camera FOV
  (if IsRunning
    (bind (_direction _movecameratrack) (`Timeline|T_MoveCamera` :!label _label_3)
      (:`Update`
        (`CameraComponent.SetFieldOfView` (`self.FirstPersonCamera`) _movecameratrack)))
    (else
      (goto _label_3 :!via `Reverse`))))

(event `InputAction|Crouch`
  (params (Key :type "Key Structure"))
  ;[1 1 1] Crouch Controls
  (:`Pressed`
    (if (`NavMovementComponent.IsMovingOnGround` (`self.CharacterMovement`))
      (`self.Crouch`)
      (else
        (`self.UnCrouch` :!label _label_4))))
  (:`Released`
    (goto _label_4)))

(event `InputAction|Jump`
  (params (Key :type "Key Structure"))
  ;[1 1 1] Jump Controls
  (:`Pressed`
    (if (`NavMovementComponent.IsMovingOnGround` (`self.CharacterMovement`))
      (`self.Jump`))))

(fn `ShowInGameHUD`
  (`/Engine/EditorBlueprintResources/StandardMacros.IsValid` (`self.In-Game HUD`)
    (:`Is Valid`
      _)
    (:`Is Not Valid`
      (bind _returnvalue (`|CreateWidget` "/Game/Widgets/WBP_In-Game_HUD.WBP_In-Game_HUD_C" (`self.PlayerController`)))
      (bind _output_get (set `self.In-Game HUD` _returnvalue))))
  (`UserWidget.AddToViewport` _output_get 0)
  (return))

(fn `UserConstructionScript`)