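; Parent room Blueprint for prototype level generation, with three wall segments per compass side and at most one door on each side.
; On BeginPlay it groups the segments into per-side arrays and randomly picks each side's door slot.
; UpdateWalls tags the chosen segment on active sides, then swaps every segment to a door or wall mesh by tag.
; A separate event shows a yellow indicator sprite while the room's objective is active.
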(event `self.ReceiveBeginPlay`
  (`self.CreateWallArrays`)
  (`self.GetRandomDoors`))

(event `UpdateWalls`
  (`self.SetWallTags`)
  (`self.SetDoors`))

(event `CheckObjectiveIndicator`
  (if (`self.ObjectiveActive`)
    (`PaperSpriteComponent.SetSpriteColor` (`self.ObjectiveIndicator`) (struct :`R` 1.0 :`G` 1.0 :`A` 1.0))
    (else
      (`PaperSpriteComponent.SetSpriteColor` :`self` (`self.ObjectiveIndicator`)))))

(fn `CreateWallArrays`
  (set `self.N_Walls` (`|MakeArray` (`self.N_Wall_1`) (`self.N_Wall_2`) (`self.N_Wall_3`)))
  (set `self.E_Walls` (`|MakeArray` (`self.E_Wall_1`) (`self.E_Wall_2`) (`self.E_Wall_3`)))
  (set `self.S_Walls` (`|MakeArray` (`self.S_Wall_1`) (`self.S_Wall_2`) (`self.S_Wall_3`)))
  (set `self.W_Walls` (`|MakeArray` (`self.W_Wall_1`) (`self.W_Wall_2`) (`self.W_Wall_3`)))
  (`KismetArrayLibrary.Array_Clear` (`self.Walls`))
  (for _array_element (`self.N_Walls`)
    (`KismetArrayLibrary.Array_Add` (`self.Walls`) _array_element))
  (for _array_element_2 (`self.E_Walls`)
    (`KismetArrayLibrary.Array_Add` (`self.Walls`) _array_element_2))
  (for _array_element_3 (`self.S_Walls`)
    (`KismetArrayLibrary.Array_Add` (`self.Walls`) _array_element_3))
  (for _array_element_4 (`self.W_Walls`)
    (`KismetArrayLibrary.Array_Add` (`self.Walls`) _array_element_4)))

(fn `GetRandomDoors`
  (set `self.N_Door` (`KismetMathLibrary.RandomIntegerInRange` 1 (`KismetArrayLibrary.Array_Length` (`self.N_Walls`))))
  (set `self.E_Door` (`KismetMathLibrary.RandomIntegerInRange` 1 (`KismetArrayLibrary.Array_Length` (`self.E_Walls`))))
  (set `self.S_Door` (`KismetMathLibrary.RandomIntegerInRange` 1 (`KismetArrayLibrary.Array_Length` (`self.S_Walls`))))
  (set `self.W_Door` (`KismetMathLibrary.RandomIntegerInRange` 1 (`KismetArrayLibrary.Array_Length` (`self.W_Walls`)))))

(fn `PickRandomDoors`
  (locals (BlankTags :type "Array of Name") (DoorTags :type "Array of Name") (TempRandomNumber :type Integer))
  (for _array_element (`self.N_Walls`)
    (set `ActorComponent.ComponentTags` (`local.BlankTags`) _array_element))
  (bind _output_get (set `local.TempRandomNumber` (`KismetMathLibrary.RandomIntegerInRange` 0 (- (`KismetArrayLibrary.Array_Length` (`self.N_Walls`)) 1))))
  (set `ActorComponent.ComponentTags` (`local.DoorTags`) (`|GetArrayItem` (`self.N_Walls`) _output_get))
  (set `self.N_Door` (+ (`local.TempRandomNumber`) 1))
  (for _array_element_2 (`self.E_Walls`)
    (set `ActorComponent.ComponentTags` (`local.BlankTags`) _array_element_2))
  (bind _output_get_2 (set `local.TempRandomNumber` (`KismetMathLibrary.RandomIntegerInRange` 0 (- (`KismetArrayLibrary.Array_Length` (`self.E_Walls`)) 1))))
  (set `ActorComponent.ComponentTags` (`local.DoorTags`) (`|GetArrayItem` (`self.E_Walls`) _output_get_2))
  (set `self.E_Door` (+ (`local.TempRandomNumber`) 1))
  (for _array_element_3 (`self.S_Walls`)
    (set `ActorComponent.ComponentTags` (`local.BlankTags`) _array_element_3))
  (bind _output_get_3 (set `local.TempRandomNumber` (`KismetMathLibrary.RandomIntegerInRange` 0 (- (`KismetArrayLibrary.Array_Length` (`self.S_Walls`)) 1))))
  (set `ActorComponent.ComponentTags` (`local.DoorTags`) (`|GetArrayItem` (`self.S_Walls`) _output_get_3))
  (set `self.S_Door` (+ (`local.TempRandomNumber`) 1))
  (for _array_element_4 (`self.W_Walls`)
    (set `ActorComponent.ComponentTags` (`local.BlankTags`) _array_element_4))
  (bind _output_get_4 (set `local.TempRandomNumber` (`KismetMathLibrary.RandomIntegerInRange` 0 (- (`KismetArrayLibrary.Array_Length` (`self.W_Walls`)) 1))))
  (set `ActorComponent.ComponentTags` (`local.DoorTags`) (`|GetArrayItem` (`self.W_Walls`) _output_get_4))
  (set `self.W_Door` (+ (`local.TempRandomNumber`) 1)))

(fn `SetDoors`
  (for _array_element (`self.Walls`)
    (if (`ActorComponent.ComponentHasTag` _array_element "IsDoor")
      (`StaticMeshComponent.SetStaticMesh` _array_element "/Game/Meshes/LevelGeneration/SM_Door.SM_Door")
      (else
        (`StaticMeshComponent.SetStaticMesh` _array_element "/Game/Meshes/LevelGeneration/SM_Wall.SM_Wall")))))

(fn `SetWallTags`
  (locals (BlankTags :type "Array of Name") (DoorTags :type "Array of Name"))
  (for _array_element (`self.N_Walls`)
    (set `ActorComponent.ComponentTags` (`local.BlankTags`) _array_element))
  (if (not (not (`self.N_Door_Active`)))
    (set `ActorComponent.ComponentTags` (`local.DoorTags`) (`|GetArrayItem` (`self.N_Walls`) (- (`self.N_Door`) 1))))
  (for _array_element_2 (`self.E_Walls`)
    (set `ActorComponent.ComponentTags` (`local.BlankTags`) _array_element_2))
  (if (not (not (`self.E_Door_Active`)))
    (set `ActorComponent.ComponentTags` (`local.DoorTags`) (`|GetArrayItem` (`self.E_Walls`) (- (`self.E_Door`) 1))))
  (for _array_element_3 (`self.S_Walls`)
    (set `ActorComponent.ComponentTags` (`local.BlankTags`) _array_element_3))
  (if (not (not (`self.S_Door_Active`)))
    (set `ActorComponent.ComponentTags` (`local.DoorTags`) (`|GetArrayItem` (`self.S_Walls`) (- (`self.S_Door`) 1))))
  (for _array_element_4 (`self.W_Walls`)
    (set `ActorComponent.ComponentTags` (`local.BlankTags`) _array_element_4))
  (if (not (not (`self.W_Door_Active`)))
    (set `ActorComponent.ComponentTags` (`local.DoorTags`) (`|GetArrayItem` (`self.W_Walls`) (- (`self.W_Door`) 1)))))

(fn `UserConstructionScript`)