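; Prototype level-generation room that spawns a random mix of standard and sniper enemies when the player enters.
; BeginPlay rolls a small count for each enemy type into EnemiesToSpawn, after running the parent room's logic.
; The first player overlap with PlayerDetection fires SpawnEnemies once, placing each enemy at a random, slightly raised point within the EnemySpawnArea bounds.
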(event `self.ReceiveBeginPlay`
  (`parent.ReceiveBeginPlay`)
  (set `self.EnemiesToSpawn` (make `/Game/Blueprints/Interactions/STR_EnemyCount` (`KismetMathLibrary.RandomIntegerInRange` 1 2) (`KismetMathLibrary.RandomIntegerInRange` 1 2))))

(event `self.PlayerDetection.OnComponentBeginOverlap`
  (params (OverlappedComponent :type "PrimitiveComponent Object Reference") (OtherActor :type "Actor Object Reference") (OtherComp :type "PrimitiveComponent Object Reference") (OtherBodyIndex :type Integer) (bFromSweep :type Boolean) (SweepResult :type "HitResult Structure (by ref)"))
  (cast `/Game/Blueprints/Player/BP_Player` OtherActor)
  (`/Engine/EditorBlueprintResources/StandardMacros.DoOnce` false
    (:`Completed`
      (`self.SpawnEnemies`))))

(event `SpawnEnemies`
  (bind (_enemiestospawn_standard _enemiestospawn_sniper) (break `/Game/Blueprints/Interactions/STR_EnemyCount` (`self.EnemiesToSpawn`)))
  (bind _enemiestospawn_standard_2 (break `/Game/Blueprints/Interactions/STR_EnemyCount` (`self.EnemiesToSpawn`)))
  (bind (_origin _boxextent) (`KismetSystemLibrary.GetComponentBounds` (`self.EnemySpawnArea`)))
  (bind (_origin_2 _boxextent_2) (`KismetSystemLibrary.GetComponentBounds` (`self.EnemySpawnArea`)))
  (for _ (range 1 (+ _enemiestospawn_standard_2 1))
    (`|SpawnActorFromClass` "/Game/Blueprints/Enemies/Standard/BP_Enemy_Standard.BP_Enemy_Standard_C" (`KismetMathLibrary.MakeTransform` (+ (`KismetMathLibrary.RandomPointInBoundingBox` _origin_2 _boxextent_2) (0.0 0.0 100.0))) "Undefined" "OverrideRootScale" null null))
  (for _ (range 1 (+ _enemiestospawn_sniper 1))
    (`|SpawnActorFromClass` "/Game/Blueprints/Enemies/Sniper/BP_Enemy_Sniper.BP_Enemy_Sniper_C" (`KismetMathLibrary.MakeTransform` (+ (`KismetMathLibrary.RandomPointInBoundingBox` _origin _boxextent) (0.0 0.0 100.0))) "Undefined" "OverrideRootScale" null null)))

(fn `UserConstructionScript`
  (`parent.UserConstructionScript`))