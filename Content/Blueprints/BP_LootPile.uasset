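; BP_LootPile is an interactable pickup that grants the player health and mission loot, then destroys itself.
; On BeginPlay it caches the mission manager and player; InteractMenu then runs AddHealth, AddAmmo and GrabLoot.
; GrabLoot adds a random amount to the manager's LootCollected and shows it as player popup text.
; AddAmmo is an empty stub, and the primary and secondary weapon ammo refill logic is left disconnected.
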(event `self.ReceiveBeginPlay`
  (bind _returnvalue (`GameplayStatics.GetActorOfClass` "/Game/Blueprints/Missions/BP_MissionManager.BP_MissionManager_C"))
  (set `self.MissionManagerRef` _returnvalue)
  (bind _asbp_player (cast `/Game/Blueprints/Player/BP_Player` (`GameplayStatics.GetPlayerCharacter` 0)))
  (set `self.As BP Player` _asbp_player))

(event `GrabLoot`
  (bind _missionmanagerref (`self.MissionManagerRef`))
  (set `self.RandomLoot` (`KismetMathLibrary.RandomIntegerInRange` 4 8))
  (set `/Game/Blueprints/Missions/BP_MissionManager.LootCollected` (+ (`/Game/Blueprints/Missions/BP_MissionManager.LootCollected` _missionmanagerref) (`self.RandomLoot`)) _missionmanagerref)
  (`/Game/Blueprints/Player/BP_Player.SetPopupText` (`self.As BP Player`) (`KismetTextLibrary.Conv_StringToText` (`KismetStringLibrary.Concat_StrStr` "+" (`KismetStringLibrary.Conv_IntToString` (`self.RandomLoot`)))) 3.0)
  (`self.K2_DestroyActor`))

(event `AddHealth`
  (`/Game/Blueprints/Player/BP_Player.AdjustHealth` (`self.As BP Player`) (`KismetMathLibrary.RandomFloatInRange` 15.0 30.0) false null))

(event `AddAmmo`)

(fn `Interact_Menu`
  (params (Interactor :type "/Game/Blueprints/Player/BP_Player Object Reference"))
  (returns (`Success?` :type Boolean))
  (`self.AddHealth`)
  (`self.AddAmmo`)
  (`self.GrabLoot`)
  (return false))

(fn `UserConstructionScript`)