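; Interactable timed-objective actor that opens a menu when its required mission objective is current, passing its timer name to Command Centre menus.
; Tick polls the mission manager to switch interaction tags through paired DoOnce gates.
; StartTimer runs a looping countdown mirrored to the manager.
; Tick clears the timer at zero and advances the current objective.
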(event `self.ReceiveTick`
  (params (DeltaSeconds :type "Float (single-precision)"))
  (`self.CheckObjectiveEnabled`)
  (`self.StopTimer`))

(event `self.ReceiveBeginPlay`
  (`KismetArrayLibrary.Array_Add` (`self.InteractTags`) (`self.TimerName`))
  (`KismetArrayLibrary.Array_Add` (`self.BlankTags`) (`self.TimerName`))
  (set `self.Tags` (`self.InteractTags`))
  (bind _returnvalue (`GameplayStatics.GetActorOfClass` "/Game/Blueprints/Missions/BP_MissionManager.BP_MissionManager_C"))
  (set `self.MissionManagerRef` _returnvalue)
  (bind _asbp_player (cast `/Game/Blueprints/Player/BP_Player` (`GameplayStatics.GetPlayerCharacter` 0)))
  (set `self.As BP Player` _asbp_player))

(event `OpenMenu`
  (if (== (`/Game/Blueprints/Missions/BP_MissionManager.CurrentObjective` (`self.MissionManagerRef`)) (`self.RequiredObjective`))
    (bind _currentactivemenu (`/Game/Blueprints/Player/BP_Player.OpenMenu` (`self.As BP Player`) (`self.Menu to Open`) false))
    (set `self.Current Active Menu` _currentactivemenu)
    (`self.CheckMenuType`)))

(event `CheckMenuType`
  (if (== (`self.Menu to Open`) "/Game/Widgets/WBP_CommandCentre.WBP_CommandCentre_C")
    (bind _aswbp_command_centre (cast `/Game/Widgets/WBP_CommandCentre` (`self.Current Active Menu`)))
    (set `/Game/Widgets/WBP_CommandCentre.TimerName` (`self.TimerName`) _aswbp_command_centre)))

(event `CheckObjectiveEnabled`
  (if (== (`/Game/Blueprints/Missions/BP_MissionManager.CurrentObjective` (`self.MissionManagerRef`)) (`self.RequiredObjective`))
    (`/Engine/EditorBlueprintResources/StandardMacros.DoOnce` false :!label _label
      (:`Completed`
        (set `self.Tags` (`self.InteractTags`))
        (goto _label_2 :!via `Reset`)))
    (else
      (`/Engine/EditorBlueprintResources/StandardMacros.DoOnce` false :!label _label_2
        (:`Completed`
          (set `self.Tags` (`self.BlankTags`))
          (goto _label :!via `Reset`))))))

(event `StartTimer`
  (set `self.TimerActive` true)
  (`KismetSystemLibrary.PrintString` "Timer Started")
  (set `/Game/Blueprints/Missions/BP_MissionManager.Timer` (`self.TimerLength`) (`self.MissionManagerRef`))
  (bind _returnvalue (`KismetSystemLibrary.K2_SetTimerDelegate` (delegate `Timer Countdown`) 0.1 true))
  (set `self.TimerRef` _returnvalue))

(event `Timer Countdown`
  (bind _output_get (set `self.CurrentTimer` (- (`self.CurrentTimer`) 0.1)))
  (set `/Game/Blueprints/Missions/BP_MissionManager.CurrentTimer` _output_get (`self.MissionManagerRef`)))

(event `StopTimer`
  (if (`self.TimerActive`)
    (if (<= (`self.CurrentTimer`) 0.0)
      (`KismetSystemLibrary.K2_ClearAndInvalidateTimerHandle` (`self.TimerRef`))
      (`/Engine/EditorBlueprintResources/StandardMacros.IncrementInt` (`/Game/Blueprints/Missions/BP_MissionManager.CurrentObjective` (`self.MissionManagerRef`))
        (:`  `
          (set `self.TimerActive` false))))))

(fn `Interact_Menu`
  (params (Interactor :type "/Game/Blueprints/Player/BP_Player Object Reference"))
  (returns (`Success?` :type Boolean))
  (`self.OpenMenu`)
  (return false))

(fn `UserConstructionScript`)