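; BP_Objective_GoTo is a mission objective actor that completes a "go to location" step when the player reaches it.
; On BeginPlay it finds and caches the BP_MissionManager in the level.
; When a BP_Player overlaps its ObjectiveArea, it increments the manager's CurrentObjective, but only if that matches its RequiredObjective, so objectives advance in order.
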(event `self.ReceiveBeginPlay`
  (bind _returnvalue (`GameplayStatics.GetActorOfClass` "/Game/Blueprints/Missions/BP_MissionManager.BP_MissionManager_C"))
  (set `self.MissionManagerRef` _returnvalue))

(event `self.ObjectiveArea.OnComponentBeginOverlap`
  (params (OverlappedComponent :type "PrimitiveComponent Object Reference") (OtherActor :type "Actor Object Reference") (OtherComp :type "PrimitiveComponent Object Reference") (OtherBodyIndex :type Integer) (bFromSweep :type Boolean) (SweepResult :type "HitResult Structure (by ref)"))
  (cast `/Game/Blueprints/Player/BP_Player` OtherActor)
  (if (== (`/Game/Blueprints/Missions/BP_MissionManager.CurrentObjective` (`self.MissionManagerRef`)) (`self.RequiredObjective`))
    (`/Engine/EditorBlueprintResources/StandardMacros.IncrementInt` (`/Game/Blueprints/Missions/BP_MissionManager.CurrentObjective` (`self.MissionManagerRef`)))))

(fn `UserConstructionScript`)