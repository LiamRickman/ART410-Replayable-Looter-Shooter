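; Mission objective actor that spawns enemies when the player reaches its area and completes once they are cleared.
; On overlap during its required objective, it increments the mission manager's counter and once spawns Standard and Sniper enemies at random points within its bounds.
; Spawned enemies link back and join EnemiesToDefeat.
; Tick compares that array's length to half itself, true only when empty, then advances the mission and destroys the actor.
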(event `self.ReceiveBeginPlay`
  (bind _returnvalue (`GameplayStatics.GetActorOfClass` "/Game/Blueprints/Missions/BP_MissionManager.BP_MissionManager_C"))
  (set `self.MissionManagerRef` _returnvalue))

(event `self.ObjectiveArea.OnComponentBeginOverlap`
  (params (OverlappedComponent :type "PrimitiveComponent Object Reference") (OtherActor :type "Actor Object Reference") (OtherComp :type "PrimitiveComponent Object Reference") (OtherBodyIndex :type Integer) (bFromSweep :type Boolean) (SweepResult :type "HitResult Structure (by ref)"))
  (cast `/Game/Blueprints/Player/BP_Player` OtherActor)
  (if (== (`/Game/Blueprints/Missions/BP_MissionManager.CurrentObjective` (`self.MissionManagerRef`)) (`self.RequiredObjective`))
    (`/Engine/EditorBlueprintResources/StandardMacros.IncrementInt` (`/Game/Blueprints/Missions/BP_MissionManager.CurrentObjective` (`self.MissionManagerRef`))
      (:`  `
        (`/Engine/EditorBlueprintResources/StandardMacros.DoOnce` false
          (:`Completed`
            (`self.SpawnEnemies`)))))))

(event `SpawnEnemies`
  (bind (_enemiestospawn_standard _enemiestospawn_sniper) (break `/Game/Blueprints/Interactions/STR_EnemyCount` (`self.EnemiesToSpawn`)))
  (bind _enemiestospawn_standard_2 (break `/Game/Blueprints/Interactions/STR_EnemyCount` (`self.EnemiesToSpawn`)))
  (bind (_origin _boxextent) (`self.GetActorBounds` self false false))
  (bind (_origin_2 _boxextent_2) (`self.GetActorBounds` self false false))
  (for _ (range 1 (+ _enemiestospawn_standard_2 1))
    (bind _returnvalue (`|SpawnActorFromClass` "/Game/Blueprints/Enemies/Standard/BP_Enemy_Standard.BP_Enemy_Standard_C" (`KismetMathLibrary.MakeTransform` (+ (`KismetMathLibrary.RandomPointInBoundingBox` _origin _boxextent) (0.0 0.0 100.0))) "Undefined" "OverrideRootScale" null null))
    (set `/Game/Blueprints/Enemies/BP_Enemy_Parent.LinkedObjective` self _returnvalue)
    (`KismetArrayLibrary.Array_Add` (`self.EnemiesToDefeat`) _returnvalue))
  (for _ (range 1 (+ _enemiestospawn_sniper 1))
    (bind _returnvalue_2 (`|SpawnActorFromClass` "/Game/Blueprints/Enemies/Sniper/BP_Enemy_Sniper.BP_Enemy_Sniper_C" (`KismetMathLibrary.MakeTransform` (+ (`KismetMathLibrary.RandomPointInBoundingBox` _origin_2 _boxextent_2) (0.0 0.0 100.0))) "Undefined" "OverrideRootScale" null null))
    (set `/Game/Blueprints/Enemies/BP_Enemy_Parent.LinkedObjective` self _returnvalue_2)
    (`KismetArrayLibrary.Array_Add` (`self.EnemiesToDefeat`) _returnvalue_2)))

(event `self.ReceiveTick`
  (params (DeltaSeconds :type "Float (single-precision)"))
  (bind _returnvalue (`KismetArrayLibrary.Array_Length` (`self.EnemiesToDefeat`)))
  (if (== (`/Game/Blueprints/Missions/BP_MissionManager.CurrentObjective` (`self.MissionManagerRef`)) (+ (`self.RequiredObjective`) 1))
    (if (<= _returnvalue (/ _returnvalue 2))
      (`/Engine/EditorBlueprintResources/StandardMacros.DoOnce` false
        (:`Completed`
          (`/Game/Blueprints/Missions/BP_MissionManager.IncreaseObjective` (`self.MissionManagerRef`))
          (`self.K2_DestroyActor`))))))

(fn `UserConstructionScript`)