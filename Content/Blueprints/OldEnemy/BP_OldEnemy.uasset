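; BP_OldEnemy is a gun-wielding enemy with health that damages the player with hitscan shots.
; ShootWeapon line-traces forward from the mesh at a raised height with debug drawing, plays the pistol sound and muzzle flash, and calls AdjustHealth on a hit BP_Player.
; Its own AdjustHealth adds or subtracts clamped health, prints the value, and destroys the actor at zero.
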(event `ShootWeapon`
  (bind _mesh (`self.Mesh`))
  (bind _returnvalue (+ (`SceneComponent.K2_GetComponentLocation` _mesh) (0.0 0.0 60.0)))
  (bind _outhit (`KismetSystemLibrary.LineTraceSingle` :`Start` _returnvalue :`End` (+ _returnvalue (* (`SceneComponent.GetForwardVector` _mesh) 100000.0)) :`TraceChannel` "TraceTypeQuery1" :`DrawDebugType` "ForDuration"))
  (`|ExecutionSequence`
    (:`then_0`
      (`GameplayStatics.PlaySoundAtLocation` "/Game/StarterContent/MilitaryWeapSilver/Sound/Pistol/Cues/PistolA_Fire_Cue.PistolA_Fire_Cue" (`self.K2_GetActorLocation`) (struct) 1.0 1.0 0.0 null null null null)
      (`GameplayStatics.SpawnEmitterAttached` "/Game/StarterContent/MilitaryWeapSilver/FX/P_Pistol_MuzzleFlash_01.P_Pistol_MuzzleFlash_01" (`self.Weapon`) "Muzzle" (0.0 0.0 0.0) (struct) (1.0 1.0 1.0) "SnapToTarget"))
    (:`then_1`
      (bind _asbp_player (cast `/Game/Blueprints/Player/BP_Player` (`.HitActor` (`GameplayStatics.BreakHitResult` _outhit))))
      (`/Game/Blueprints/Player/BP_Player.AdjustHealth` _asbp_player (`self.Damage`) true null))))

(event `self.ReceiveBeginPlay`
  (set `self.CurrentHealth` (`self.MaxHealth`)))

(fn `Adjust Health`
  (params (Amount :type "Float (double-precision)") (DamageEnemy :type Boolean))
  (if DamageEnemy
    (bind _output_get (set `self.CurrentHealth` (`KismetMathLibrary.FClamp` (- (`self.CurrentHealth`) (`local.Amount`)) 0.0 (`self.MaxHealth`))))
    (else
      (set `self.CurrentHealth` (`KismetMathLibrary.FClamp` (+ (`self.CurrentHealth`) (`local.Amount`)) 0.0 (`self.MaxHealth`)))))
  (`KismetSystemLibrary.PrintString` (`KismetStringLibrary.Conv_DoubleToString` _output_get))
  (if (<= (`self.CurrentHealth`) 0.0)
    (`self.K2_DestroyActor`)))

(fn `UserConstructionScript`)