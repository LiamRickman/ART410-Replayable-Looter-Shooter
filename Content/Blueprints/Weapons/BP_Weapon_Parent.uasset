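; Parent weapon Blueprint for first-person guns, handling fire and reload input, ammo and recoil, with firing disabled in the "Ship" level.
; Fire either runs spread-randomized camera line traces that damage enemies, push physics objects and leave decals, or launches a physics grenade.
; Both paths share recoil, effects and a fire-rate delay that loops for full-auto.
; Reload refills from spare ammo on montage blend-out; aim-down-sights logic is disconnected.
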(event `self.ReceiveBeginPlay`
  (`self.EnableInput` (`GameplayStatics.GetPlayerController` 0))
  (bind _asbp_player (cast `/Game/Blueprints/Player/BP_Player` (`GameplayStatics.GetPlayerCharacter` 0)))
  (set `self.As BP Player` _asbp_player)
  (set `self.CurrentAmmo` (`self.MagSize`))
  (`/Game/Blueprints/Player/BP_Player.HidePlayerFromMinmap` (`self.As BP Player`) (`self.Weapon`)))

(event `InputAction|ADS`
  (params (Key :type "Key Structure"))
  ;[1 1 1] ADS
)

(event `InputAction|Shoot/Fire`
  (params (Key :type "Key Structure"))
  (bind _currentspread (`self.CurrentSpread`))
  (bind _as_bp_player (`self.As BP Player`))
  (bind (_shothit_bblockinghit _shothit_binitialoverlap _shothit_time _shothit_distance _shothit_location _shothit_impactpoint _shothit_normal _shothit_impactnormal _shothit_physmat _shothit_hitactor) (`GameplayStatics.BreakHitResult` (`self.ShotHit`)))
  (bind _as_bp_player_2 (`self.As BP Player`))
  (bind (_recoilvalues_location_updownmin _recoilvalues_location_updownmax _recoilvalues_location_frontbackmin _recoilvalues_location_frontbackmax _recoilvalues_rotation_updownmin _recoilvalues_rotation_updownmax _recoilvalues_rotation_tiltmin _recoilvalues_rotation_tiltmax _recoilvalues_rotation_sidemin _recoilvalues_rotation_sidemax) (break `/Game/Blueprints/Weapons/S_WeaponRecoil` (`self.RecoilValues`)))
  (bind (_recoilvalues_location_updownmin_2 _recoilvalues_location_updownmax_2 _recoilvalues_location_frontbackmin_2 _recoilvalues_location_frontbackmax_2 _recoilvalues_rotation_updownmin_2 _recoilvalues_rotation_updownmax_2 _recoilvalues_rotation_tiltmin_2 _recoilvalues_rotation_tiltmax_2 _recoilvalues_rotation_sidemin_2 _recoilvalues_rotation_sidemax_2 _recoilvalues_camerarecoilvmin _recoilvalues_camerarecoilvmax _recoilvalues_camerarecoilhmin _recoilvalues_camerarecoilhmax) (break `/Game/Blueprints/Weapons/S_WeaponRecoil` (`self.RecoilValues`)))
  (bind _returnvalue (* _currentspread -1.0))
  (bind _firstpersoncamera (`/Game/Blueprints/Player/BP_Player.FirstPersonCamera` (`self.As BP Player`)))
  (bind _returnvalue_2 (`SceneComponent.K2_GetComponentLocation` _firstpersoncamera))
  (bind (_returnvalue_roll _returnvalue_pitch _returnvalue_yaw) (`KismetMathLibrary.BreakRotator` (`SceneComponent.K2_GetComponentRotation` _firstpersoncamera)))
  (:`Pressed`
    (bind _returnvalue_3 (`GameplayStatics.GetCurrentLevelName` true))
    (if (`KismetStringLibrary.EqualEqual_StrStr` _returnvalue_3 "Ship")
      _
      (elif (not (`/Game/Blueprints/Player/BP_Player.IsMenuActive` (`self.As BP Player`)))
        (set `self.FireButtonPressed` true)
        (if (or (`self.IsReloading`) (`/Game/Blueprints/Player/BP_Player.IsSwitchingWeapons` _as_bp_player_2) (>= (`CharacterMovementComponent.MaxWalkSpeed` (`Character.CharacterMovement` _as_bp_player_2)) (`/Game/Blueprints/Player/BP_Player.SprintSpeed` _as_bp_player_2))) :!label _label
          _
          (elif (> (`self.CurrentAmmo`) 0)
            (if (`self.ReadyToShoot`)
              (set `self.ReadyToShoot` false)
              (`/Game/Animations/Player/ABP_Player.FireWeapon` (`/Game/Blueprints/Player/BP_Player.ABP Player` (`self.As BP Player`)) (`KismetMathLibrary.MakeTransform` (`KismetMathLibrary.MakeVector` 0.0 (`KismetMathLibrary.RandomFloatInRange` _recoilvalues_location_updownmin _recoilvalues_location_updownmax) (`KismetMathLibrary.RandomFloatInRange` _recoilvalues_location_frontbackmin _recoilvalues_location_frontbackmax)) (`KismetMathLibrary.MakeRotator` (`KismetMathLibrary.RandomFloatInRange` _recoilvalues_rotation_updownmin _recoilvalues_rotation_updownmax) (`KismetMathLibrary.RandomFloatInRange` _recoilvalues_rotation_tiltmin _recoilvalues_rotation_tiltmax) (`KismetMathLibrary.RandomFloatInRange` _recoilvalues_rotation_sidemin _recoilvalues_rotation_sidemax))))
              (if (`self.GrenadeLauncher`)
                (`self.FireGrenadeLauncher`)
                (else
                  (if (> (`self.NoOfShots`) 0)
                    (set `self.CurrentSpread` (`self.Spread`))
                    (else
                      (set `self.CurrentSpread` 0.0)))
                  (for _ (range 1 (+ (`self.NoOfShots`) 1))
                    (bind (_outhit _returnvalue_4) (`KismetSystemLibrary.LineTraceSingle` _returnvalue_2 (+ _returnvalue_2 (* (`KismetMathLibrary.GetForwardVector` (`KismetMathLibrary.MakeRotator` _returnvalue_roll (+ _returnvalue_pitch (`KismetMathLibrary.RandomFloatInRange` _returnvalue _currentspread)) (+ _returnvalue_yaw (`KismetMathLibrary.RandomFloatInRange` _returnvalue _currentspread)))) 100000)) "TraceTypeQuery1"))
                    (if _returnvalue_4
                      (set `self.ShotHit` _outhit)
                      (bind (_bblockinghit _binitialoverlap _time _distance _location _impactpoint _normal _impactnormal _physmat _hitactor _hitcomponent) (`GameplayStatics.BreakHitResult` _outhit))
                      (`GameplayStatics.SpawnEmitterAtLocation` "/Game/StarterContent/MilitaryWeapSilver/FX/P_Impact_Metal_Medium_01.P_Impact_Metal_Medium_01" _impactpoint (`KismetMathLibrary.Conv_VectorToRotator` _impactnormal))
                      (bind (_returnvalue_roll_2 _returnvalue_pitch_2 _returnvalue_yaw_2) (`KismetMathLibrary.BreakRotator` (`KismetMathLibrary.Conv_VectorToRotator` _impactnormal)))
                      (`GameplayStatics.SpawnDecalAttached` "/Game/Decals/M_BulletHole.M_BulletHole" (1.0 25.0 25.0) _hitcomponent "None" _impactpoint (`KismetMathLibrary.MakeRotator` (`KismetMathLibrary.RandomFloatInRange` 0.0 359.0) _returnvalue_pitch_2 _returnvalue_yaw_2) "KeepWorldPosition" 5.0)
                      (if (`SceneComponent.IsSimulatingPhysics` (`Actor.RootComponent` _hitactor) "None")
                        (`PrimitiveComponent.AddImpulseAtLocation` _hitcomponent (* (`KismetMathLibrary.GetForwardVector` (`SceneComponent.K2_GetComponentRotation` (`/Game/Blueprints/Player/BP_Player.FirstPersonCamera` (`self.As BP Player`)))) 100000.0) _location "None"))
                      (if (`KismetMathLibrary.ClassIsChildOf` (`GameplayStatics.GetObjectClass` _shothit_hitactor) "/Game/Blueprints/Enemies/BP_Enemy_Parent.BP_Enemy_Parent_C")
                        (bind _asbp_enemy_parent (cast `/Game/Blueprints/Enemies/BP_Enemy_Parent` _shothit_hitactor))
                        (`/Game/Blueprints/Enemies/BP_Enemy_Parent.Adjust Health` _asbp_enemy_parent (`self.Damage`) true))))
                  (`Pawn.AddControllerPitchInput` _as_bp_player (`KismetMathLibrary.RandomFloatInRange` _recoilvalues_camerarecoilvmin _recoilvalues_camerarecoilvmax) :!label _label_2)
                  (`Pawn.AddControllerYawInput` _as_bp_player (`KismetMathLibrary.RandomFloatInRange` _recoilvalues_camerarecoilhmin _recoilvalues_camerarecoilhmax))
                  (`GameplayStatics.PlaySound2D` (`self.ShotSFX`) 1.0 1.0 0.0 null null)
                  (`GameplayStatics.SpawnEmitterAttached` "/Game/StarterContent/MilitaryWeapSilver/FX/P_Pistol_MuzzleFlash_01.P_Pistol_MuzzleFlash_01" (`self.Weapon`) "Muzzle" (0.0 0.0 0.0) (struct) (1.0 1.0 1.0) "SnapToTarget")
                  (`/Engine/EditorBlueprintResources/StandardMacros.DecrementInt` (`self.CurrentAmmo`)
                    (:`  `
                      (`KismetSystemLibrary.Delay` (`self.FireRate`))
                      (set `self.ReadyToShoot` true)
                      (`/Game/Animations/Player/ABP_Player.StopFireWeapon` (`/Game/Blueprints/Player/BP_Player.ABP Player` (`self.As BP Player`)))
                      (if (`self.IsFullAuto`)
                        (if (`self.FireButtonPressed`)
                          (goto _label)))))))))))))
  (:`Released`
    (set `self.FireButtonPressed` false)))

(event `InputAction|Reload`
  (params (Key :type "Key Structure"))
  (:`Pressed`
    (if (`/Game/Blueprints/Player/BP_Player.IsMenuActive` (`self.As BP Player`))
      _
      (elif (and (> (`self.SpareAmmo`) 0) (< (`self.CurrentAmmo`) (`self.MagSize`)))
        (if (not (or (`self.IsReloading`) (`/Game/Blueprints/Player/BP_Player.IsSwitchingWeapons` (`self.As BP Player`))))
          (set `self.IsReloading` true)
          (`|PlayMontage` (`/Game/Blueprints/Player/BP_Player.Arms` (`self.As BP Player`)) "/Game/Animations/Player/Primaries/AssaultRifle/AM_AssaultRifle_Lower.AM_AssaultRifle_Lower"
            (:`then`
              (`GameplayStatics.PlaySound2D` "/Game/StarterContent/MilitaryWeapSilver/Sound/Rifle/Cues/Rifle_Reload_Cue.Rifle_Reload_Cue" 1.0 1.0 0.0 null null))
            (:`OnBlendOut`
              (set `self.IsReloading` false)
              (set `self.AmmoDifference` (- (`self.MagSize`) (`self.CurrentAmmo`)))
              (if (>= (`self.SpareAmmo`) (`self.AmmoDifference`))
                (set `self.CurrentAmmo` (`self.MagSize`))
                (set `self.SpareAmmo` (- (`self.SpareAmmo`) (`self.AmmoDifference`)))
                (else
                  (set `self.CurrentAmmo` (+ (`self.CurrentAmmo`) (`self.SpareAmmo`)))
                  (set `self.SpareAmmo` 0))))))))))

(event `FireGrenadeLauncher`
  (if (not (`/Game/Blueprints/Player/BP_Player.IsMenuActive` (`self.As BP Player`)))
    (bind _returnvalue (`|SpawnActorFromClass` "/Game/Blueprints/Weapons/Grenades/BP_Grenade_Impact.BP_Grenade_Impact_C" (`KismetMathLibrary.MakeTransform` (`SceneComponent.GetSocketLocation` (`self.Weapon`) "Muzzle") (`KismetMathLibrary.MakeRotator` (`KismetMathLibrary.RandomFloatInRange` 0.0 359.0) (`KismetMathLibrary.RandomFloatInRange` 0.0 359.0) (`KismetMathLibrary.RandomFloatInRange` 0.0 359.0))) "Undefined" "OverrideRootScale" null null))
    (`PrimitiveComponent.SetPhysicsLinearVelocity` (`/Game/Blueprints/Weapons/Grenades/BP_Grenade_Parent.SM_Grenade` _returnvalue) (* (`KismetMathLibrary.GetForwardVector` (`SceneComponent.K2_GetComponentRotation` (`/Game/Blueprints/Player/BP_Player.FirstPersonCamera` (`self.As BP Player`)))) 3000.0) false "None")
    (goto _label_2)))

(fn `UserConstructionScript`)