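; LMG weapon Blueprint that swaps the scope material on its Weapon mesh while the aim button is held.
; Tick checks IsAimButtonPressed, applying the main scope material when pressed and the scope body material otherwise.
; Two DoOnce nodes reset each other, so each swap runs only when the aim state changes.
; BeginPlay and the construction script only call their parent versions.
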(event `self.ReceiveBeginPlay`
  (`parent.ReceiveBeginPlay`))

(event `self.ReceiveTick`
  (params (DeltaSeconds :type "Float (single-precision)"))
  (if (`self.IsAimButtonPressed`)
    (`/Engine/EditorBlueprintResources/StandardMacros.DoOnce` false :!label _label
      (:`Completed`
        (`PrimitiveComponent.SetMaterial` (`self.Weapon`) 4 "/Game/Materials/Weapons/LMG/M_LMG_Scope_Main.M_LMG_Scope_Main")
        (goto _label_2 :!via `Reset`)))
    (else
      (`/Engine/EditorBlueprintResources/StandardMacros.DoOnce` false :!label _label_2
        (:`Completed`
          (`PrimitiveComponent.SetMaterial` (`self.Weapon`) 4 "/Game/Materials/Weapons/LMG/M_LMG_Scope_Body.M_LMG_Scope_Body")
          (goto _label :!via `Reset`))))))

(fn `UserConstructionScript`
  (`parent.UserConstructionScript`))