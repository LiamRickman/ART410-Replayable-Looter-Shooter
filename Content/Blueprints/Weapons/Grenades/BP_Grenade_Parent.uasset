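; Parent grenade Blueprint that detonates either on a fuse timer or on impact, depending on DetonateOnImpact.
; Molotov variants spawn BP_Molotov on detonation; others apply radius damage through overlap queries, with players taking half the damage enemies take.
; Non-molotov detonation also spawns an explosion and GrenadeCount cluster grenades launched upward with randomized velocities.
; The grenade destroys itself after detonating.
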(event `self.ReceiveBeginPlay`
  (if (not (`self.DetonateOnImpact`))
    (`KismetSystemLibrary.K2_SetTimerDelegate` (delegate `Detonate`) (`self.FuseTime`))))

(event `Detonate`
  (if (`self.IsMolotov`)
    (`|SpawnActorFromClass` "/Game/Blueprints/Weapons/Grenades/BP_Molotov.BP_Molotov_C" (`KismetMathLibrary.MakeTransform` (`SceneComponent.K2_GetComponentLocation` (`self.SM_Grenade`))) "Undefined" "OverrideRootScale" null null)
    (`self.K2_DestroyActor`)
    (else
      (`self.ApplyDamage`)
      (`|SpawnActorFromClass` "/Game/Blueprints/Weapons/Grenades/BP_Explosion.BP_Explosion_C" (`SceneComponent.K2_GetComponentToWorld` (`self.SM_Grenade`)) "Undefined" "OverrideRootScale" null null)
      (for _ (range 1 (+ (`self.GrenadeCount`) 1))
        (bind _returnvalue (`|SpawnActorFromClass` "/Game/Blueprints/Weapons/Grenades/BP_Grenade_Cluster.BP_Grenade_Cluster_C" (`KismetMathLibrary.MakeTransform` (`SceneComponent.K2_GetComponentLocation` (`self.SM_Grenade`))) "Undefined" "OverrideRootScale" null null))
        (`PrimitiveComponent.SetPhysicsLinearVelocity` (`/Game/Blueprints/Weapons/Grenades/BP_Grenade_Parent.SM_Grenade` _returnvalue) (`KismetMathLibrary.MakeVector` (`KismetMathLibrary.RandomFloatInRange` -50.0 50.0) (`KismetMathLibrary.RandomFloatInRange` -50.0 50.0) (`KismetMathLibrary.RandomFloatInRange` 600.0 1000.0)) false "None"))
      (`self.K2_DestroyActor`))))

(event `self.SM_Grenade.OnComponentHit`
  (params (HitComponent :type "PrimitiveComponent Object Reference") (OtherActor :type "Actor Object Reference") (OtherComp :type "PrimitiveComponent Object Reference") (NormalImpulse :type "Vector Structure") (Hit :type "HitResult Structure (by ref)"))
  (if (`self.DetonateOnImpact`)
    (`self.Detonate`)))

(fn `ApplyDamage`
  (for _array_element (`PrimitiveComponent.GetOverlappingActors` (`self.ExplosionRadius`) "/Game/Blueprints/Player/BP_Player.BP_Player_C")
    (bind _asbp_player (cast `/Game/Blueprints/Player/BP_Player` _array_element))
    (`/Game/Blueprints/Player/BP_Player.AdjustHealth` _asbp_player (/ (`self.ExplosionDamage`) 2.0) true)
    (`KismetSystemLibrary.PrintString` "Player Damaged"))
  (for _array_element_2 (`PrimitiveComponent.GetOverlappingActors` (`self.ExplosionRadius`) "/Game/Blueprints/Enemies/BP_Enemy.BP_Enemy_C")
    (bind _asbp_enemy (cast `/Game/Blueprints/Enemies/BP_Enemy` _array_element_2))
    (`/Game/Blueprints/Enemies/BP_Enemy.Adjust Health` _asbp_enemy (`self.ExplosionDamage`) true)
    (`KismetSystemLibrary.PrintString` "Enemy Damaged"))
  (return))

(fn `UserConstructionScript`)