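; Molotov fire area that damages the player and BP_OldEnemy actors standing inside it.
; BeginPlay plays smash and fire sounds and sizes DamageRange; after its lifespan, a fade-out timeline rescales the range, then destroys the actor.
; DamageRange overlaps start or stop a looping player-damage timer and maintain an enemy array.
; Tick uses a DoOnce to run one shared damage timer while that array is non-empty.
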(event `self.ReceiveTick`
  (params (DeltaSeconds :type "Float (single-precision)"))
  (if (> (`KismetArrayLibrary.Array_Length` (`self.EnemiesToDamage`)) 0)
    (`/Engine/EditorBlueprintResources/StandardMacros.DoOnce` false :!label _label
      (:`Completed`
        (bind _returnvalue (`KismetSystemLibrary.K2_SetTimerDelegate` (delegate `DamageEnemiesLoop`) 0.5 true))
        (set `self.DamageEnemyTimer` _returnvalue)))
    (else
      (`KismetSystemLibrary.K2_ClearAndInvalidateTimerHandle` (`self.DamageEnemyTimer`))
      (goto _label :!via `Reset`))))

(event `DamageEnemiesLoop`
  (for _array_element (`self.EnemiesToDamage`)
    (`/Game/Blueprints/OldEnemy/BP_OldEnemy.Adjust Health` _array_element 5.0 true)))

(event `self.ReceiveBeginPlay`
  (bind _molotovsize (`self.MolotovSize`))
  (`GameplayStatics.PlaySoundAtLocation` "/Game/SFX/Weapons/SC_Molotov_Smash.SC_Molotov_Smash" (`SceneComponent.K2_GetComponentLocation` (`self.DefaultSceneRoot`)) (struct) 1.0 1.0 1.0 "/Game/StarterContent/MilitaryWeapSilver/Sound/Attenuation/Explosion_att.Explosion_att" null null null)
  (bind _returnvalue (`GameplayStatics.SpawnSoundAtLocation` "/Game/StarterContent/Audio/Fire01_Cue.Fire01_Cue" (`self.K2_GetActorLocation`) (struct) 1.0 1.0 0.0 null null))
  (`SceneComponent.SetWorldScale3D` (`self.DamageRange`) (`KismetMathLibrary.MakeVector` _molotovsize _molotovsize 1.0))
  (bind _asbp_player (cast `/Game/Blueprints/Player/BP_Player` (`GameplayStatics.GetPlayerCharacter` 0)))
  (set `self.As BP Player` _asbp_player)
  (`KismetSystemLibrary.Delay` (`self.MolotovLIfeSpan`))
  (`AudioComponent.Stop` _returnvalue)
  (bind (_direction _timeout) (`Timeline|MolotovFadeOut`)
    (:`Update`
      (bind _returnvalue_2 (* _timeout (`self.MolotovSize`)))
      (`SceneComponent.SetWorldScale3D` (`self.DamageRange`) (`KismetMathLibrary.MakeVector` _returnvalue_2 _returnvalue_2 1.0)))
    (:`Finished`
      (`self.K2_DestroyActor`))))

(event `self.DamageRange.OnComponentBeginOverlap`
  (params (OverlappedComponent :type "PrimitiveComponent Object Reference") (OtherActor :type "Actor Object Reference") (OtherComp :type "PrimitiveComponent Object Reference") (OtherBodyIndex :type Integer) (bFromSweep :type Boolean) (SweepResult :type "HitResult Structure (by ref)"))
  (bind _returnvalue (`GameplayStatics.GetObjectClass` OtherActor))
  (if (== _returnvalue "/Game/Blueprints/Player/BP_Player.BP_Player_C")
    (`self.StartDamagePlayer`)
    (`KismetSystemLibrary.PrintString` "Player Enter"))
  (if (== _returnvalue "/Game/Blueprints/OldEnemy/BP_OldEnemy.BP_OldEnemy_C")
    (bind _asbp_old_enemy (cast `/Game/Blueprints/OldEnemy/BP_OldEnemy` OtherActor))
    (`KismetArrayLibrary.Array_Add` (`self.EnemiesToDamage`) _asbp_old_enemy)))

(event `self.DamageRange.OnComponentEndOverlap`
  (params (OverlappedComponent :type "PrimitiveComponent Object Reference") (OtherActor :type "Actor Object Reference") (OtherComp :type "PrimitiveComponent Object Reference") (OtherBodyIndex :type Integer))
  (bind _returnvalue (`GameplayStatics.GetObjectClass` OtherActor))
  (if (== _returnvalue "/Game/Blueprints/Player/BP_Player.BP_Player_C")
    (`self.StopDamagePlayer`)
    (`KismetSystemLibrary.PrintString` "Player Leave"))
  (if (== _returnvalue "/Game/Blueprints/OldEnemy/BP_OldEnemy.BP_OldEnemy_C")
    (bind _asbp_old_enemy (cast `/Game/Blueprints/OldEnemy/BP_OldEnemy` OtherActor))
    (`KismetArrayLibrary.Array_RemoveItem` (`self.EnemiesToDamage`) _asbp_old_enemy)))

(event `StartDamagePlayer`
  (bind _returnvalue (`KismetSystemLibrary.K2_SetTimerDelegate` (delegate `DamagePlayerLoop`) 0.5 true))
  (set `self.DamagePlayerTimer` _returnvalue))

(event `DamagePlayerLoop`
  (`/Game/Blueprints/Player/BP_Player.AdjustHealth` (`self.As BP Player`) 5.0 true null))

(event `StopDamagePlayer`
  (`KismetSystemLibrary.K2_ClearAndInvalidateTimerHandle` (`self.DamagePlayerTimer`)))

(fn `UserConstructionScript`)