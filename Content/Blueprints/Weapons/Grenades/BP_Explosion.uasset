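; BP_Explosion is a grenade explosion actor that applies a radial force impulse and plays an explosion sound when it spawns.
; BeginPlay fires the RadialForce component, plays the cue at the root's location, then sets a short lifespan.
; An unconnected branch would set the force radius from ExplosionRange, but it never runs.
; CalculateDamage only returns the distance from a hit actor to the explosion and is not called here.
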(event `self.ReceiveBeginPlay`
  (`RadialForceComponent.FireImpulse` (`self.RadialForce`))
  (`GameplayStatics.PlaySoundAtLocation` "/Game/StarterContent/Audio/Explosion_Cue.Explosion_Cue" (`SceneComponent.K2_GetComponentLocation` (`self.DefaultSceneRoot`)) (struct) 1.0 1.0 0.0 null null null null)
  (`self.SetLifeSpan` 3.0))

(fn `CalculateDamage`
  (params (HitActor :type "Actor Object Reference"))
  (returns (Damage :type "Float (double-precision)"))
  (return (`KismetMathLibrary.Vector_Distance` (`self.K2_GetActorLocation` HitActor) (`SceneComponent.K2_GetComponentLocation` (`self.DefaultSceneRoot`)))))

(fn `UserConstructionScript`)