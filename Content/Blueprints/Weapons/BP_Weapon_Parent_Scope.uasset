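; Parent Blueprint for a scoped player weapon, handling input-driven firing, ammo and reload, with a scope camera attached at a socket.
; Firing line-traces per shot from AimSocket with spread, spawns impacts and decals, applies animation and camera recoil, and loops after FireRate for full-auto.
; Reload picks rifle or revolver montages by the player's weapon ID and refills ammo on blend-out.
; ADS blending, scope toggling and muzzle flash logic are disconnected.
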(event `self.ReceiveBeginPlay`
  (`self.EnableInput` (`GameplayStatics.GetPlayerController` 0))
  (bind _asbp_player (cast `/Game/Blueprints/BP_Player` (`GameplayStatics.GetPlayerCharacter` 0)))
  (set `self.As BP Player` _asbp_player)
  (set `self.CurrentAmmo` (`self.MaxAmmo`))
  (`SceneComponent.K2_AttachToComponent` (`self.ScopeCamera`) (`self.Weapon`) "ScopeSocket" "SnapToTarget" "KeepRelative" "KeepRelative" true))

(event `EnableScopeCamera`
  (`SceneComponent.SetVisibility` (`self.ScopeCamera`) true false))

(event `DisableScopeCamera`
  (`SceneComponent.SetVisibility` (`self.ScopeCamera`) false false))

(event `InputAction|ADS`
  (params (Key :type "Key Structure"))
  ;[1 1 1] ADS
)

(event `InputAction|Shoot/Fire`
  (params (Key :type "Key Structure"))
  (bind _currentspread (`self.CurrentSpread`))
  (bind _as_bp_player (`self.As BP Player`))
  (bind _weapon (`self.Weapon`))
  (bind (_recoilvalues_location_updownmin _recoilvalues_location_updownmax _recoilvalues_location_frontbackmin _recoilvalues_location_frontbackmax _recoilvalues_rotation_updownmin _recoilvalues_rotation_updownmax _recoilvalues_rotation_tiltmin _recoilvalues_rotation_tiltmax _recoilvalues_rotation_sidemin _recoilvalues_rotation_sidemax) (break `/Game/Blueprints/Weapons/S_WeaponRecoil` (`self.RecoilValues`)))
  (bind (_recoilvalues_location_updownmin_2 _recoilvalues_location_updownmax_2 _recoilvalues_location_frontbackmin_2 _recoilvalues_location_frontbackmax_2 _recoilvalues_rotation_updownmin_2 _recoilvalues_rotation_updownmax_2 _recoilvalues_rotation_tiltmin_2 _recoilvalues_rotation_tiltmax_2 _recoilvalues_rotation_sidemin_2 _recoilvalues_rotation_sidemax_2 _recoilvalues_camerarecoilvmin _recoilvalues_camerarecoilvmax _recoilvalues_camerarecoilhmin _recoilvalues_camerarecoilhmax) (break `/Game/Blueprints/Weapons/S_WeaponRecoil` (`self.RecoilValues`)))
  (bind _returnvalue (`SceneComponent.GetSocketLocation` _weapon "AimSocket"))
  (bind (_returnvalue_roll _returnvalue_pitch _returnvalue_yaw) (`KismetMathLibrary.BreakRotator` (`SceneComponent.GetSocketRotation` _weapon "AimSocket")))
  (bind _returnvalue_2 (* _currentspread -1.0))
  (:`Pressed`
    (set `self.FireButtonPressed` true)
    (if (or (`self.IsReloading`) (`/Game/Blueprints/BP_Player.IsSwitchingWeapons` (`self.As BP Player`))) :!label _label
      _
      (elif (> (`self.CurrentAmmo`) 0)
        (if (`self.ReadyToShoot`)
          (set `self.ReadyToShoot` false)
          (`/Game/Animations/Player/ABP_Player.FireWeapon` (`/Game/Blueprints/BP_Player.ABP Player` (`self.As BP Player`)) (`KismetMathLibrary.MakeTransform` (`KismetMathLibrary.MakeVector` 0.0 (`KismetMathLibrary.RandomFloatInRange` _recoilvalues_location_updownmin _recoilvalues_location_updownmax) (`KismetMathLibrary.RandomFloatInRange` _recoilvalues_location_frontbackmin _recoilvalues_location_frontbackmax)) (`KismetMathLibrary.MakeRotator` (`KismetMathLibrary.RandomFloatInRange` _recoilvalues_rotation_updownmin _recoilvalues_rotation_updownmax) (`KismetMathLibrary.RandomFloatInRange` _recoilvalues_rotation_tiltmin _recoilvalues_rotation_tiltmax) (`KismetMathLibrary.RandomFloatInRange` _recoilvalues_rotation_sidemin _recoilvalues_rotation_sidemax))))
          (if (> (`self.NoOfShots`) 0)
            (set `self.CurrentSpread` (`self.Spread`))
            (else
              (set `self.CurrentSpread` 0.0)))
          (for _ (range 1 (+ (`self.NoOfShots`) 1))
            (bind _outhit (`KismetSystemLibrary.LineTraceSingle` _returnvalue (+ _returnvalue (* (`KismetMathLibrary.GetForwardVector` (`KismetMathLibrary.MakeRotator` _returnvalue_roll (+ _returnvalue_pitch (`KismetMathLibrary.RandomFloatInRange` _returnvalue_2 _currentspread)) (+ _returnvalue_yaw (`KismetMathLibrary.RandomFloatInRange` _returnvalue_2 _currentspread)))) 100000)) "TraceTypeQuery1"))
            (bind (_bblockinghit _binitialoverlap _time _distance _location _impactpoint _normal _impactnormal _physmat _hitactor _hitcomponent) (`GameplayStatics.BreakHitResult` _outhit))
            (`GameplayStatics.SpawnEmitterAtLocation` "/Game/StarterContent/MilitaryWeapSilver/FX/P_Impact_Metal_Medium_01.P_Impact_Metal_Medium_01" _impactpoint (`KismetMathLibrary.Conv_VectorToRotator` _impactnormal))
            (bind (_returnvalue_roll_2 _returnvalue_pitch_2 _returnvalue_yaw_2) (`KismetMathLibrary.BreakRotator` (`KismetMathLibrary.Conv_VectorToRotator` _impactnormal)))
            (`GameplayStatics.SpawnDecalAttached` "/Game/Decals/M_BulletHole.M_BulletHole" (10.0 25.0 25.0) _hitcomponent "None" _impactpoint (`KismetMathLibrary.MakeRotator` (`KismetMathLibrary.RandomFloatInRange` 0.0 359.0) _returnvalue_pitch_2 _returnvalue_yaw_2) "KeepWorldPosition" 5.0))
          (`Pawn.AddControllerPitchInput` _as_bp_player (`KismetMathLibrary.RandomFloatInRange` _recoilvalues_camerarecoilvmin _recoilvalues_camerarecoilvmax))
          (`Pawn.AddControllerYawInput` _as_bp_player (`KismetMathLibrary.RandomFloatInRange` _recoilvalues_camerarecoilhmin _recoilvalues_camerarecoilhmax))
          (`GameplayStatics.PlaySound2D` (`self.ShotSFX`) 1.0 1.0 0.0 null null)
          (`/Engine/EditorBlueprintResources/StandardMacros.DecrementInt` (`self.CurrentAmmo`)
            (:`  `
              (`KismetSystemLibrary.Delay` (`self.FireRate`))
              (set `self.ReadyToShoot` true)
              (`/Game/Animations/Player/ABP_Player.StopFireWeapon` (`/Game/Blueprints/BP_Player.ABP Player` (`self.As BP Player`)))
              (if (`self.IsFullAuto`)
                (if (`self.FireButtonPressed`)
                  (goto _label)))))))))
  (:`Released`
    (set `self.FireButtonPressed` false)))

(event `InputAction|Reload`
  (params (Key :type "Key Structure"))
  (:`Pressed`
    (if (not (`self.IsReloading`))
      (set `self.IsReloading` true)
      (if (== (`/Game/Blueprints/BP_Player.CurrentWeaponID` (`self.As BP Player`)) 1)
        (`|PlayMontage` (`/Game/Blueprints/BP_Player.Arms` (`self.As BP Player`)) "/Game/Animations/Player/Primaries/_Old/AssaultRifle_Old/AM_AssaultRifle_Reload_Old.AM_AssaultRifle_Reload_Old"
          (:`then`
            (`SkeletalMeshComponent.PlayAnimation` (`self.Weapon`) "/Game/Animations/Weapons/Primaries/AssaultRifle/AS_AssaultRifle_Reload_Gun.AS_AssaultRifle_Reload_Gun" false))
          (:`OnBlendOut`
            (set `self.IsReloading` false)
            (set `self.CurrentAmmo` (`self.MaxAmmo`))))
        (else
          (`|PlayMontage` (`/Game/Blueprints/BP_Player.Arms` (`self.As BP Player`)) "/Game/Animations/Player/Secondaries/_Old/AM_Revolver_Old_Reload.AM_Revolver_Old_Reload"
            (:`then`
              (`SkeletalMeshComponent.PlayAnimation` (`self.Weapon`) "/Game/Animations/Weapons/Secondaries/Revolver_Old/AS_Revolver_Old_Reload_Gun.AS_Revolver_Old_Reload_Gun" false))
            (:`OnBlendOut`
              (set `self.IsReloading` false)
              (set `self.CurrentAmmo` (`self.MaxAmmo`)))))))))

(fn `UserConstructionScript`)