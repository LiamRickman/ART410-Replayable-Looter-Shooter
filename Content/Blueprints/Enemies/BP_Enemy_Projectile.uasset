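; BP_Enemy_Projectile is a projectile fired by enemies that damages the player on impact.
; When its Projectile component hits the player, it applies its Damage through the player's AdjustHealth and destroys itself.
; On any other hit it destroys itself, except when it strikes another enemy projectile or its own BulletOwner, which it ignores.
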(event `self.Projectile.OnComponentHit`
  (params (HitComponent :type "PrimitiveComponent Object Reference") (OtherActor :type "Actor Object Reference") (OtherComp :type "PrimitiveComponent Object Reference") (NormalImpulse :type "Vector Structure") (Hit :type "HitResult Structure (by ref)"))
  (bind _returnvalue (`GameplayStatics.GetObjectClass` OtherActor))
  (if (== _returnvalue "/Game/Blueprints/Player/BP_Player.BP_Player_C")
    (bind _asbp_player (cast `/Game/Blueprints/Player/BP_Player` OtherActor))
    (`/Game/Blueprints/Player/BP_Player.AdjustHealth` _asbp_player (`self.Damage`) true)
    (`self.K2_DestroyActor`)
    (elif (not (or (== _returnvalue "BP_Enemy_Projectile_C") (== OtherActor (`self.BulletOwner`))))
      (`self.K2_DestroyActor`))))

(fn `UserConstructionScript`)