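; Enemy homing missile that detonates to damage the player within its explosion radius.
; After a brief arming delay, it spawns a target actor at the player's current position and homes on that actor rather than the player.
; It detonates near the target or on hitting anything but another missile, unless invincible.
; Detonation damages overlapping BP_Player actors, spawns an explosion and destroys both missile and target.
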(event `self.ReceiveBeginPlay`
  (bind _projectilemovement (`self.ProjectileMovement`))
  (`KismetSystemLibrary.Delay` 0.1)
  (`ParticleSystemComponent.SetTemplate` (`self.ParticleSystem`) "/Game/StarterContent/MilitaryWeapSilver/FX/P_RocketLauncher_Trail_01.P_RocketLauncher_Trail_01")
  (set `self.Invincible` false)
  (bind _returnvalue (`|SpawnActorFromClass` "/Game/Blueprints/Enemies/BP_Homing_Missile_Target.BP_Homing_Missile_Target_C" (`self.GetTransform` (`GameplayStatics.GetPlayerCharacter` 0)) "Undefined" "OverrideRootScale" null null))
  (bind _output_get (set `self.Target` _returnvalue))
  (set `ProjectileMovementComponent.HomingTargetComponent` (`Actor.RootComponent` _output_get) _projectilemovement)
  (set `ProjectileMovementComponent.bIsHomingProjectile` true _projectilemovement)
  (set `ProjectileMovementComponent.HomingAccelerationMagnitude` 10000.0 _projectilemovement))

(event `Detonate`
  (if (!= (`GameplayStatics.GetObjectClass` (stale `self.Sphere.OnComponentHit` OtherActor)) "BP_Homing_Missile_C") :!label _label
    (if (not (`self.Invincible`))
      (`self.ApplyDamage`)
      (`|SpawnActorFromClass` "/Game/Blueprints/Weapons/Grenades/BP_Explosion.BP_Explosion_C" (`SceneComponent.K2_GetComponentToWorld` (`self.Sphere`)) "Undefined" "OverrideRootScale" null null)
      (`self.K2_DestroyActor`)
      (`self.K2_DestroyActor` (`self.Target`)))))

(event `self.Sphere.OnComponentHit`
  (params (HitComponent :type "PrimitiveComponent Object Reference") (OtherActor :type "Actor Object Reference") (OtherComp :type "PrimitiveComponent Object Reference") (NormalImpulse :type "Vector Structure") (Hit :type "HitResult Structure (by ref)"))
  (goto _label))

(event `self.ReceiveTick`
  (params (DeltaSeconds :type "Float (single-precision)"))
  (`/Engine/EditorBlueprintResources/StandardMacros.IsValid` (`self.Target`)
    (:`Is Valid`
      (if (<= (`KismetMathLibrary.Vector_Distance` (`self.K2_GetActorLocation`) (`self.K2_GetActorLocation` (`self.Target`))) 20.0)
        (`self.Detonate`)))))

(fn `ApplyDamage`
  (for _array_element (`PrimitiveComponent.GetOverlappingActors` (`self.ExplosionRadius`) "/Game/Blueprints/Player/BP_Player.BP_Player_C")
    (bind _asbp_player (cast `/Game/Blueprints/Player/BP_Player` _array_element))
    (`/Game/Blueprints/Player/BP_Player.AdjustHealth` _asbp_player (`self.ExplosionDamage`) true)
    (`KismetSystemLibrary.PrintString` "Player Damaged")))

(fn `UserConstructionScript`)