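; BP_Enemy is an enemy actor with a health pool that starts at MaxHealth on BeginPlay.
; Adjust Health subtracts or adds an amount depending on the DamageEnemy flag, clamping the result between zero and MaxHealth.
; It prints the new health for debugging and destroys the actor when health reaches zero.
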(event `self.ReceiveBeginPlay`
  (set `self.CurrentHealth` (`self.MaxHealth`)))

(fn `Adjust Health`
  (params (Amount :type "Float (double-precision)") (DamageEnemy :type Boolean))
  (if DamageEnemy
    (bind _output_get (set `self.CurrentHealth` (`KismetMathLibrary.FClamp` (- (`self.CurrentHealth`) (`local.Amount`)) 0.0 (`self.MaxHealth`))))
    (else
      (set `self.CurrentHealth` (`KismetMathLibrary.FClamp` (+ (`self.CurrentHealth`) (`local.Amount`)) 0.0 (`self.MaxHealth`)))))
  (`KismetSystemLibrary.PrintString` (`KismetStringLibrary.Conv_DoubleToString` _output_get))
  (if (<= (`self.CurrentHealth`) 0.0)
    (`self.K2_DestroyActor`)))

(fn `UserConstructionScript`)