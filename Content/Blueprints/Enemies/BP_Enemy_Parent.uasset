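; Base enemy Blueprint that spawns its AI controller, tracks clamped health and destroys itself at zero.
; It provides callable attacks: delayed bursts of projectiles aimed at the player, homing missiles alternating between two spawn points, and a laser.
; The laser fades body emissive via timelines, then line-traces toward the player each tick to place its Niagara beam end, running a looping damage timer while hitting.
; SetEnemyState is an empty switch here.
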(event `SetEnemyState`
  (params (`New State` :type "/Game/Blueprints/Enemies/ENUM_EnemyStates Enum" :default "NewEnumerator0"))
  (switch `/Game/Blueprints/Enemies/ENUM_EnemyStates` `New State`))

(event `self.ReceiveBeginPlay`
  (set `self.AIControllerClass` (`self.EnemyAIController`))
  (set `self.CurrentHealth` (`self.MaxHealth`))
  (`self.SpawnDefaultController`)
  (`self.StopLaser`)
  (bind _asbp_player (cast `/Game/Blueprints/Player/BP_Player` (`GameplayStatics.GetPlayerCharacter` 0)))
  (set `self.As BP Player` _asbp_player))

(event `ShootBullet`
  (params (Bullets :type Integer) (Delay :type "Float (double-precision)"))
  (bind _output_get (set `self.BulletsToFire` Bullets))
  (if (> _output_get 0) :!label _label
    (bind _returnvalue (`|SpawnActorFromClass` "/Game/Blueprints/Enemies/BP_Enemy_Projectile.BP_Enemy_Projectile_C" (`SceneComponent.K2_GetComponentToWorld` (`self.BulletSpawn`)) "Undefined" "OverrideRootScale" null null))
    (set `/Game/Blueprints/Enemies/BP_Enemy_Projectile.BulletOwner` self _returnvalue)
    (`PrimitiveComponent.SetPhysicsLinearVelocity` (`/Game/Blueprints/Enemies/BP_Enemy_Projectile.Projectile` _returnvalue) (* (`KismetMathLibrary.Normal` (`KismetMathLibrary.GetForwardVector` (`KismetMathLibrary.FindLookAtRotation` (`self.K2_GetActorLocation`) (`self.K2_GetActorLocation` (`GameplayStatics.GetPlayerCharacter` 0))))) 2500.0) false "None")
    (`KismetSystemLibrary.Delay` Delay)
    (set `self.BulletsToFire` (- (`self.BulletsToFire`) 1))
    (goto _label)))

(event `ShootHomingMissile`
  (params (Missiles :type Integer) (Delay :type "Float (double-precision)"))
  (bind _missilespawn1 (`self.MissileSpawn1`))
  (bind _missilespawn2 (`self.MissileSpawn2`))
  (bind (_returnvalue_roll _returnvalue_pitch _returnvalue_yaw) (`KismetMathLibrary.BreakRotator` (`SceneComponent.K2_GetComponentRotation` _missilespawn1)))
  (bind (_returnvalue_roll_2 _returnvalue_pitch_2 _returnvalue_yaw_2) (`KismetMathLibrary.BreakRotator` (`SceneComponent.K2_GetComponentRotation` _missilespawn2)))
  (bind _output_get (set `self.MissilesToFire` Missiles))
  (if (> _output_get 0) :!label _label_2
    (switch `int` (`self.CurrentMissileSpawn`)
      (:`1`
        (set `self.CurrentMissileSpawn` 2)
        (`|SpawnActorFromClass` "/Game/Blueprints/Enemies/BP_Homing_Missile.BP_Homing_Missile_C" (`KismetMathLibrary.MakeTransform` (`SceneComponent.K2_GetComponentLocation` _missilespawn1) (`KismetMathLibrary.MakeRotator` _returnvalue_roll _returnvalue_pitch _returnvalue_yaw)) "Undefined" "OverrideRootScale" null null))
      (:`2`
        (set `self.CurrentMissileSpawn` 1)
        (`|SpawnActorFromClass` "/Game/Blueprints/Enemies/BP_Homing_Missile.BP_Homing_Missile_C" (`KismetMathLibrary.MakeTransform` (`SceneComponent.K2_GetComponentLocation` _missilespawn2) (`KismetMathLibrary.MakeRotator` _returnvalue_roll_2 _returnvalue_pitch_2 _returnvalue_yaw_2)) "Undefined" "OverrideRootScale" null null)))
    (`KismetSystemLibrary.Delay` Delay)
    (set `self.MissilesToFire` (- (`self.MissilesToFire`) 1))
    (goto _label_2)))

(event `StartLaser`
  (bind (_direction _emissive_value) (`Timeline|LaserEmissive` :!via `PlayFromStart`)
    (:`Update`
      (`MeshComponent.SetScalarParameterValueOnMaterials` (`self.Body`) "Emissive" _emissive_value))
    (:`Finished`
      (set `self.LaserActive` true)
      (`FXSystemComponent.SetColorParameter` (`self.Laser`) "User.Color" (struct :`R` 10.0 :`A` 1.0)))))

(event `StopLaser`
  (set `self.LaserHittingPlayer` false)
  (set `self.LaserActive` false)
  (`FXSystemComponent.SetColorParameter` (`self.Laser`) "User.Color" (struct :`R` 10.0))
  (bind (_direction _emissive_value) (`Timeline|LaserEmissive_2` :!via `PlayFromStart`)
    (:`Update`
      (`MeshComponent.SetScalarParameterValueOnMaterials` (`self.Body`) "Emissive" _emissive_value))))

(event `self.ReceiveTick`
  (params (DeltaSeconds :type "Float (single-precision)"))
  (`self.UpdateLaser`)
  (if (`self.LaserHittingPlayer`)
    (`/Engine/EditorBlueprintResources/StandardMacros.DoOnce` false :!label _label_3
      (:`Completed`
        (bind _returnvalue (`KismetSystemLibrary.K2_SetTimerDelegate` (delegate `DamagePlayer_Laser`) 0.1 true))
        (set `self.LaserDamageTimer` _returnvalue)))
    (else
      (`KismetSystemLibrary.K2_ClearAndInvalidateTimerHandle` (`self.LaserDamageTimer`))
      (goto _label_3 :!via `Reset`))))

(event `DamagePlayer_Laser`
  (`/Game/Blueprints/Player/BP_Player.AdjustHealth` (`self.As BP Player`) 5.0 true))

(fn `Adjust Health`
  (params (Amount :type "Float (double-precision)") (DamageEnemy :type Boolean))
  (if DamageEnemy
    (bind _output_get (set `self.CurrentHealth` (`KismetMathLibrary.FClamp` (- (`self.CurrentHealth`) (`local.Amount`)) 0.0 (`self.MaxHealth`))))
    (else
      (set `self.CurrentHealth` (`KismetMathLibrary.FClamp` (+ (`self.CurrentHealth`) (`local.Amount`)) 0.0 (`self.MaxHealth`)))))
  (`KismetSystemLibrary.PrintString` (`KismetStringLibrary.Conv_DoubleToString` _output_get))
  (if (<= (`self.CurrentHealth`) 0.0)
    (`self.K2_DestroyActor`)))

(fn `UpdateLaser`
  (if (`self.LaserActive`)
    (bind (_outhit _returnvalue) (`KismetSystemLibrary.LineTraceSingle` (`SceneComponent.K2_GetComponentLocation` (`self.Laser`)) (`self.K2_GetActorLocation` (`GameplayStatics.GetPlayerCharacter` 0)) "TraceTypeQuery2"))
    (if _returnvalue
      (bind (_bblockinghit _binitialoverlap _time _distance _location _impactpoint _normal _impactnormal _physmat _hitactor) (`GameplayStatics.BreakHitResult` _outhit))
      (`FXSystemComponent.SetVectorParameter` (`self.Laser`) "User.Beam End" (+ _location (0.0 0.0 25.0)))
      (if (== (`GameplayStatics.GetObjectClass` _hitactor) "/Game/Blueprints/Player/BP_Player.BP_Player_C")
        (set `self.LaserHittingPlayer` true)
        (else
          (set `self.LaserHittingPlayer` false))))
    (else
      (`KismetSystemLibrary.K2_ClearAndInvalidateTimerHandle` (`self.LaserDamageTimer`)))))

(fn `UserConstructionScript`)