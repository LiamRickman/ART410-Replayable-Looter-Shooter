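; Player animation posing Blueprint that displays a character and weapon and derives the weapon's aim socket offset for the current pose.
; UpdateAnimData swaps both skeletal meshes and plays the given pose animation looping on the character.
; GetNewAimSocket returns the location and rotation of the weapon's AimSocket relative to the character's ik_hand_root socket.
; The event graph and construction script hold no logic, so both functions rely on external callers.
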(fn `GetNewAimSocket`
  (returns (`Return Value Location` :type "Vector Structure") (`Return Value Rotation` :type "Rotator Structure"))
  (bind (_returnvalue_location _returnvalue_rotation) (`KismetMathLibrary.BreakTransform` (`KismetMathLibrary.MakeRelativeTransform` (`SceneComponent.GetSocketTransform` (`self.WeaponMesh`) "AimSocket" "RTS_World") (`SceneComponent.GetSocketTransform` (`self.Mesh`) "ik_hand_root" "RTS_World"))))
  (return _returnvalue_location _returnvalue_rotation))

(fn `UpdateAnimData`
  (params (CharacterMesh :type "SkeletalMesh Object Reference") (WeaponMesh :type "SkeletalMesh Object Reference") (PoseAnimation :type "AnimationAsset Object Reference"))
  (bind _mesh (`self.Mesh`))
  (`SkinnedMeshComponent.SetSkinnedAssetAndUpdate` _mesh CharacterMesh true)
  (`SkeletalMeshComponent.SetAnimation` _mesh PoseAnimation)
  (`SkeletalMeshComponent.Play` _mesh true)
  (`SkinnedMeshComponent.SetSkinnedAssetAndUpdate` (`self.WeaponMesh`) WeaponMesh true)
  (return))

(fn `UserConstructionScript`)