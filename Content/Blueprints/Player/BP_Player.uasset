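; First-person player character handling movement, look, sprint FOV, crouch, jump, HUD, and pausing menus.
; A per-tick camera trace feeds the Interact input, which messages loadout-tagged BPI_Interact actors.
; Debug numpad keys swap eight weapons between lower/raise montages, changing the child actor class and updating animation data through a level-found BP_Player_Switch.
; BeginPlay restores location from BP_Save_Main; SaveMain stores it but is not called here.
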(event `self.ReceiveBeginPlay`
  (`KismetSystemLibrary.Delay` 0.1)
  (set `self.PlayerController` (`GameplayStatics.GetPlayerController` 0))
  (`self.ShowInGameHUD`)
  (set `self.CurrentAmmo` (`self.MaxAmmo`))
  (bind _asabp_player (cast `/Game/Animations/Player/ABP_Player` (`SkeletalMeshComponent.GetAnimInstance` (`self.Arms`))))
  (set `self.ABP Player` _asabp_player)
  (bind _outactors (`GameplayStatics.GetAllActorsOfClass` "/Game/Blueprints/Player/BP_Player_Switch.BP_Player_Switch_C"))
  (set `self.BP Player Switch` (`|GetArrayItem` _outactors))
  (`self.LoadMain`))

(event `Update Weapon UI`
  ;[1 1 1] Update Weapon UI
  (`self.UpdateWeaponUI` :!label _label))

(event `InteractCheck`
  (bind _firstpersoncamera (`self.FirstPersonCamera`))
  (bind _returnvalue (`SceneComponent.K2_GetComponentLocation` _firstpersoncamera))
  (bind (_outhit _returnvalue_2) (`KismetSystemLibrary.LineTraceSingle` _returnvalue (+ _returnvalue (* (`SceneComponent.GetForwardVector` _firstpersoncamera) 250.0)) "TraceTypeQuery1"))
  (bind _output_get (set `self.InteractTraceHit` _outhit))
  (set `self.HasInteractTraceHit` _returnvalue_2)
  (set `self.CanInteract` (`KismetSystemLibrary.DoesImplementInterface` (`.HitActor` (`GameplayStatics.BreakHitResult` _output_get)) "/Game/Blueprints/BPI_Interact.BPI_Interact_C")))

(event `Key|G`
  (params (Key :type "Key Structure"))
  (:`Pressed`
    (goto _label)))

(event `TogglePauseMenu`
  (bind _returnvalue (`GameplayStatics.GetPlayerController` 0))
  (bind _pausemenuref (`self.PauseMenuRef`))
  ;[1 1 1] Pause Menu
  (if (not (`self.MenuActive?`)) :!label _label_2
    (`/Engine/EditorBlueprintResources/StandardMacros.IsValid` (`self.PauseMenuRef`)
      (:`Is Valid`
        _)
      (:`Is Not Valid`
        (bind _returnvalue_2 (`|CreateWidget` "/Game/Widgets/Menus/WBP_Menu_Pause.WBP_Menu_Pause_C"))
        (set `self.PauseMenuRef` _returnvalue_2)))
    (if (`GameplayStatics.IsGamePaused`)
      (`Widget.RemoveFromParent` _pausemenuref)
      (`GameplayStatics.SetGamePaused` false)
      (set `PlayerController.bShowMouseCursor` false _returnvalue)
      (`WidgetBlueprintLibrary.SetInputMode_GameOnly` _returnvalue)
      (set `self.PauseMenuRef` null)
      (else
        (`UserWidget.AddToViewport` _pausemenuref 0)
        (`GameplayStatics.SetGamePaused` true)
        (set `PlayerController.bShowMouseCursor` true _returnvalue)
        (`WidgetBlueprintLibrary.SetInputMode_GameAndUIEx` _returnvalue (`self.PauseMenuRef`) "LockInFullscreen")))))

(event `InputAction|Pause` :paused true
  (params (Key :type "Key Structure"))
  ;[1 1 1] Pause Menu
  (:`Pressed`
    (goto _label_2)))

(event `InputAction|Interact`
  (params (Key :type "Key Structure"))
  (:`Pressed`
    (if (`self.HasInteractTraceHit`)
      (bind _output_get (set `self.InteractHitActor` (`.HitActor` (`GameplayStatics.BreakHitResult` (`self.InteractTraceHit`)))))
      (if (`KismetSystemLibrary.DoesImplementInterface` _output_get "/Game/Blueprints/BPI_Interact.BPI_Interact_C")
        (if (`self.ActorHasTag` (`self.InteractHitActor`) "Interact_Loadout")
          (message `/Game/Blueprints/BPI_Interact.Interact_Loadout` (`self.InteractHitActor`) self))))))

(event `self.ReceiveTick`
  (params (DeltaSeconds :type "Float (single-precision)"))
  (`self.InteractCheck`))

(event `ToggleLoadoutMenu`
  (bind _returnvalue (`GameplayStatics.GetPlayerController` 0))
  (bind _loadoutmenuref (`self.LoadoutMenuRef`))
  ;[1 1 1] Loadout Menu
  (`/Engine/EditorBlueprintResources/StandardMacros.IsValid` (`self.LoadoutMenuRef`)
    (:`Is Valid`
      _)
    (:`Is Not Valid`
      (bind _returnvalue_2 (`|CreateWidget` "/Game/Widgets/Loadout/WBP_Loadout_Main.WBP_Loadout_Main_C"))
      (set `self.LoadoutMenuRef` _returnvalue_2)))
  (if (`GameplayStatics.IsGamePaused`)
    (`Widget.RemoveFromParent` _loadoutmenuref)
    (`GameplayStatics.SetGamePaused` false)
    (set `PlayerController.bShowMouseCursor` false _returnvalue)
    (`WidgetBlueprintLibrary.SetInputMode_GameOnly` _returnvalue)
    (set `self.LoadoutMenuRef` null)
    (else
      (`UserWidget.AddToViewport` _loadoutmenuref 0)
      (`GameplayStatics.SetGamePaused` true)
      (set `PlayerController.bShowMouseCursor` true _returnvalue)
      (`WidgetBlueprintLibrary.SetInputMode_GameAndUIEx` _returnvalue (`self.LoadoutMenuRef`) "LockInFullscreen"))))

(event `InputAxis|Forward/Back`
  (params (AxisValue :type "Float (single-precision)"))
  (bind (_returnvalue_roll _returnvalue_pitch _returnvalue_yaw) (`KismetMathLibrary.BreakRotator` (`self.GetControlRotation`)))
  ;[1 1 1] Movement Controls
  (bind _output_get (set `self.BS_MoveFwd` AxisValue))
  (`self.AddMovementInput` (`KismetMathLibrary.GetForwardVector` (`KismetMathLibrary.MakeRotator` 0.0 0.0 _returnvalue_yaw)) _output_get))

(event `InputAxis|Left/Right`
  (params (AxisValue :type "Float (single-precision)"))
  (bind (_returnvalue_roll _returnvalue_pitch _returnvalue_yaw) (`KismetMathLibrary.BreakRotator` (`self.GetControlRotation`)))
  ;[1 1 1] Movement Controls
  (bind _output_get (set `self.BS_MoveRight` AxisValue))
  (`self.AddMovementInput` (`KismetMathLibrary.GetRightVector` (`KismetMathLibrary.MakeRotator` 0.0 0.0 _returnvalue_yaw)) _output_get))

(event `InputAxis|LookUp/Down`
  (params (AxisValue :type "Float (single-precision)"))
  ;[1 1 1] Mouse Controls
  (bind _output_get (set `self.BS_LookUp` (* AxisValue (`self.MouseSens`))))
  (`self.AddControllerPitchInput` _output_get))

(event `InputAxis|LookLeft/Right`
  (params (AxisValue :type "Float (single-precision)"))
  ;[1 1 1] Mouse Controls
  (bind _output_get (set `self.BS_LookRight` (* AxisValue (`self.MouseSens`))))
  (`self.AddControllerYawInput` _output_get))

(event `InputAction|Sprint`
  (params (Key :type "Key Structure"))
  (bind _charactermovement (`self.CharacterMovement`))
  ;[1 1 1] Sprint Controls
  (:`Pressed`
    (set `CharacterMovementComponent.MaxWalkSpeed` (`self.SprintSpeed`) _charactermovement)
    (`self.SprintCamera` true))
  (:`Released`
    (set `CharacterMovementComponent.MaxWalkSpeed` (`self.WalkSpeed`) _charactermovement)
    (`self.SprintCamera` false)))

(event `SprintCamera`
  (params (IsRunning :type Boolean))
  ;[1 1 1] Sprint Camera FOV
  (if IsRunning
    (bind (_direction _movecameratrack) (`Timeline|T_MoveCamera` :!label _label_3)
      (:`Update`
        (`CameraComponent.SetFieldOfView` (`self.FirstPersonCamera`) _movecameratrack)))
    (else
      (goto _label_3 :!via `Reverse`))))

(event `Key|NumPadOne`
  (params (Key :type "Key Structure"))
  ;[1 1 1] Debug Weapon Switching
  (:`Pressed`
    (if (`self.IsSwitchingWeapons`)
      _
      (elif (!= (`self.CurrentWeaponID`) 1)
        (set `self.IsSwitchingWeapons` true)
        (`|PlayMontage` (`self.Arms`) "/Game/Animations/Player/Primaries/AssaultRifle/AM_AssaultRifle_Lower.AM_AssaultRifle_Lower"
          (:`OnBlendOut`
            (`ChildActorComponent.SetChildActorClass` (`self.Weapon`) "/Game/Blueprints/Weapons/Primaries/BP_Weapon_AssaultRifle.BP_Weapon_AssaultRifle_C")
            (`/Game/Blueprints/Player/BP_Player_Switch.UpdateAnimData` (`self.BP Player Switch`) "/Game/Meshes/Player/SK_Player.SK_Player" "/Game/Meshes/Weapons/Primaries/AssaultRifle/SK_AssaultRifle.SK_AssaultRifle" "/Game/Animations/Player/Primaries/AssaultRifle/AS_AssaultRifle_Pose.AS_AssaultRifle_Pose")
            (set `self.CurrentWeaponID` 1)
            (`self.Update Weapon UI`)
            (`|PlayMontage` (`self.Arms`) "/Game/Animations/Player/Primaries/AssaultRifle/AM_AssaultRifle_Raise.AM_AssaultRifle_Raise"
              (:`OnCompleted`
                (set `self.IsSwitchingWeapons` false)))))))))

(event `InputAction|Crouch`
  (params (Key :type "Key Structure"))
  ;[1 1 1] Crouch Controls
  (:`Pressed`
    (if (`NavMovementComponent.IsMovingOnGround` (`self.CharacterMovement`))
      (`self.Crouch`)
      (else
        (`self.UnCrouch` :!label _label_4))))
  (:`Released`
    (goto _label_4)))

(event `Key|NumPadTwo`
  (params (Key :type "Key Structure"))
  ;[1 1 1] Debug Weapon Switching
  (:`Pressed`
    (if (`self.IsSwitchingWeapons`)
      _
      (elif (!= (`self.CurrentWeaponID`) 2)
        (set `self.IsSwitchingWeapons` true)
        (`|PlayMontage` (`self.Arms`) "/Game/Animations/Player/Primaries/AssaultRifle/AM_AssaultRifle_Lower.AM_AssaultRifle_Lower"
          (:`OnBlendOut`
            (`ChildActorComponent.SetChildActorClass` (`self.Weapon`) "/Game/Blueprints/Weapons/Primaries/BP_Weapon_Shotgun.BP_Weapon_Shotgun_C")
            (`/Game/Blueprints/Player/BP_Player_Switch.UpdateAnimData` (`self.BP Player Switch`) "/Game/Meshes/Player/SK_Player.SK_Player" "/Game/Meshes/Weapons/Primaries/Shotgun/SK_Shotgun.SK_Shotgun" "/Game/Animations/Player/Primaries/Shotgun/AS_Shotgun_Pose.AS_Shotgun_Pose")
            (set `self.CurrentWeaponID` 2)
            (`self.Update Weapon UI`)
            (`|PlayMontage` (`self.Arms`) "/Game/Animations/Player/Primaries/AssaultRifle/AM_AssaultRifle_Raise.AM_AssaultRifle_Raise"
              (:`OnCompleted`
                (set `self.IsSwitchingWeapons` false)))))))))

(event `InputAction|Jump`
  (params (Key :type "Key Structure"))
  ;[1 1 1] Jump Controls
  (:`Pressed`
    (if (`NavMovementComponent.IsMovingOnGround` (`self.CharacterMovement`))
      (`self.Jump`))))

(event `Key|NumPadThree`
  (params (Key :type "Key Structure"))
  ;[1 1 1] Debug Weapon Switching
  (:`Pressed`
    (if (`self.IsSwitchingWeapons`)
      _
      (elif (!= (`self.CurrentWeaponID`) 3)
        (set `self.IsSwitchingWeapons` true)
        (`|PlayMontage` (`self.Arms`) "/Game/Animations/Player/Primaries/AssaultRifle/AM_AssaultRifle_Lower.AM_AssaultRifle_Lower"
          (:`OnBlendOut`
            (`ChildActorComponent.SetChildActorClass` (`self.Weapon`) "/Game/Blueprints/Weapons/Primaries/BP_Weapon_LMG.BP_Weapon_LMG_C")
            (`/Game/Blueprints/Player/BP_Player_Switch.UpdateAnimData` (`self.BP Player Switch`) "/Game/Meshes/Player/SK_Player.SK_Player" "/Game/Meshes/Weapons/Primaries/Shotgun/SK_Shotgun.SK_Shotgun" "/Game/Animations/Player/Primaries/LMG/AS_LMG_Pose.AS_LMG_Pose")
            (set `self.CurrentWeaponID` 3)
            (`self.Update Weapon UI`)
            (`|PlayMontage` (`self.Arms`) "/Game/Animations/Player/Primaries/AssaultRifle/AM_AssaultRifle_Raise.AM_AssaultRifle_Raise"
              (:`OnCompleted`
                (set `self.IsSwitchingWeapons` false)))))))))

(event `Key|NumPadFour`
  (params (Key :type "Key Structure"))
  ;[1 1 1] Debug Weapon Switching
  (:`Pressed`
    (if (`self.IsSwitchingWeapons`)
      _
      (elif (!= (`self.CurrentWeaponID`) 4)
        (set `self.IsSwitchingWeapons` true)
        (`|PlayMontage` (`self.Arms`) "/Game/Animations/Player/Primaries/AssaultRifle/AM_AssaultRifle_Lower.AM_AssaultRifle_Lower"
          (:`OnBlendOut`
            (`ChildActorComponent.SetChildActorClass` (`self.Weapon`) "/Game/Blueprints/Weapons/Primaries/BP_Weapon_GrenadeLauncher.BP_Weapon_GrenadeLauncher_C")
            (`/Game/Blueprints/Player/BP_Player_Switch.UpdateAnimData` (`self.BP Player Switch`) "/Game/Meshes/Player/SK_Player.SK_Player" "/Game/Meshes/Weapons/Primaries/GrenadeLauncher/SK_GrenadeLauncher.SK_GrenadeLauncher" "/Game/Animations/Player/Primaries/GrenadeLauncher/AS_GrenadeLauncher_Pose.AS_GrenadeLauncher_Pose")
            (set `self.CurrentWeaponID` 4)
            (`self.Update Weapon UI`)
            (`|PlayMontage` (`self.Arms`) "/Game/Animations/Player/Primaries/AssaultRifle/AM_AssaultRifle_Raise.AM_AssaultRifle_Raise"
              (:`OnCompleted`
                (set `self.IsSwitchingWeapons` false)))))))))

(event `Key|NumPadFive`
  (params (Key :type "Key Structure"))
  ;[1 1 1] Debug Weapon Switching
  (:`Pressed`
    (if (`self.IsSwitchingWeapons`)
      _
      (elif (!= (`self.CurrentWeaponID`) 5)
        (set `self.IsSwitchingWeapons` true)
        (`|PlayMontage` (`self.Arms`) "/Game/Animations/Player/Primaries/AssaultRifle/AM_AssaultRifle_Lower.AM_AssaultRifle_Lower"
          (:`OnBlendOut`
            (`ChildActorComponent.SetChildActorClass` (`self.Weapon`) "/Game/Blueprints/Weapons/Secondaries/BP_Weapon_Pistol.BP_Weapon_Pistol_C")
            (`/Game/Blueprints/Player/BP_Player_Switch.UpdateAnimData` (`self.BP Player Switch`) "/Game/Meshes/Player/SK_Player.SK_Player" "/Game/Meshes/Weapons/Secondaries/Pistol/SK_Pistol.SK_Pistol" "/Game/Animations/Player/Secondaries/Pistol/AS_Pistol_Pose.AS_Pistol_Pose")
            (set `self.CurrentWeaponID` 5)
            (`self.Update Weapon UI`)
            (`|PlayMontage` (`self.Arms`) "/Game/Animations/Player/Primaries/AssaultRifle/AM_AssaultRifle_Raise.AM_AssaultRifle_Raise"
              (:`OnCompleted`
                (set `self.IsSwitchingWeapons` false)))))))))

(event `Key|NumPadSix`
  (params (Key :type "Key Structure"))
  ;[1 1 1] Debug Weapon Switching
  (:`Pressed`
    (if (`self.IsSwitchingWeapons`)
      _
      (elif (!= (`self.CurrentWeaponID`) 6)
        (set `self.IsSwitchingWeapons` true)
        (`|PlayMontage` (`self.Arms`) "/Game/Animations/Player/Primaries/AssaultRifle/AM_AssaultRifle_Lower.AM_AssaultRifle_Lower"
          (:`OnBlendOut`
            (`ChildActorComponent.SetChildActorClass` (`self.Weapon`) "/Game/Blueprints/Weapons/Secondaries/BP_Weapon_SMG.BP_Weapon_SMG_C")
            (`/Game/Blueprints/Player/BP_Player_Switch.UpdateAnimData` (`self.BP Player Switch`) "/Game/Meshes/Player/SK_Player.SK_Player" "/Game/Meshes/Weapons/Secondaries/SMG/SK_SMG.SK_SMG" "/Game/Animations/Player/Secondaries/SMG/AS_SMG_Pose.AS_SMG_Pose")
            (set `self.CurrentWeaponID` 6)
            (`self.Update Weapon UI`)
            (`|PlayMontage` (`self.Arms`) "/Game/Animations/Player/Primaries/AssaultRifle/AM_AssaultRifle_Raise.AM_AssaultRifle_Raise"
              (:`OnCompleted`
                (set `self.IsSwitchingWeapons` false)))))))))

(event `Key|NumPadSeven`
  (params (Key :type "Key Structure"))
  ;[1 1 1] Debug Weapon Switching
  (:`Pressed`
    (if (`self.IsSwitchingWeapons`)
      _
      (elif (!= (`self.CurrentWeaponID`) 7)
        (set `self.IsSwitchingWeapons` true)
        (`|PlayMontage` (`self.Arms`) "/Game/Animations/Player/Primaries/AssaultRifle/AM_AssaultRifle_Lower.AM_AssaultRifle_Lower"
          (:`OnBlendOut`
            (`ChildActorComponent.SetChildActorClass` (`self.Weapon`) "/Game/Blueprints/Weapons/Secondaries/BP_Weapon_DoubleBarrelShotgun.BP_Weapon_DoubleBarrelShotgun_C")
            (`/Game/Blueprints/Player/BP_Player_Switch.UpdateAnimData` (`self.BP Player Switch`) "/Game/Meshes/Player/SK_Player.SK_Player" "/Game/Meshes/Weapons/Secondaries/DShotgun/SK_DShotgun.SK_DShotgun" "/Game/Animations/Player/Secondaries/DShotgun/AS_DShotgun_Pose.AS_DShotgun_Pose")
            (set `self.CurrentWeaponID` 7)
            (`self.Update Weapon UI`)
            (`|PlayMontage` (`self.Arms`) "/Game/Animations/Player/Primaries/AssaultRifle/AM_AssaultRifle_Raise.AM_AssaultRifle_Raise"
              (:`OnCompleted`
                (set `self.IsSwitchingWeapons` false)))))))))

(event `Key|NumPadEight`
  (params (Key :type "Key Structure"))
  ;[1 1 1] Debug Weapon Switching
  (:`Pressed`
    (if (`self.IsSwitchingWeapons`)
      _
      (elif (!= (`self.CurrentWeaponID`) 8)
        (set `self.IsSwitchingWeapons` true)
        (`|PlayMontage` (`self.Arms`) "/Game/Animations/Player/Primaries/AssaultRifle/AM_AssaultRifle_Lower.AM_AssaultRifle_Lower"
          (:`OnBlendOut`
            (`ChildActorComponent.SetChildActorClass` (`self.Weapon`) "/Game/Blueprints/Weapons/Secondaries/BP_Weapon_Revolver.BP_Weapon_Revolver_C")
            (`/Game/Blueprints/Player/BP_Player_Switch.UpdateAnimData` (`self.BP Player Switch`) "/Game/Meshes/Player/SK_Player.SK_Player" "/Game/Meshes/Weapons/Secondaries/Revolver/SK_Revolver.SK_Revolver" "/Game/Animations/Player/Secondaries/Revolver/AS_Revolver_Pose.AS_Revolver_Pose")
            (set `self.CurrentWeaponID` 8)
            (`self.Update Weapon UI`)
            (`|PlayMontage` (`self.Arms`) "/Game/Animations/Player/Primaries/AssaultRifle/AM_AssaultRifle_Raise.AM_AssaultRifle_Raise"
              (:`OnCompleted`
                (set `self.IsSwitchingWeapons` false)))))))))

(fn `LoadMain`
  (bind _returnvalue (`GameplayStatics.DoesSaveGameExist` (`self.SaveMainName`)))
  (if _returnvalue
    (bind _returnvalue_2 (`GameplayStatics.LoadGameFromSlot` (`self.SaveMainName`)))
    (set `self.SaveMainRef` _returnvalue_2)
    (else
      (bind _returnvalue_3 (`GameplayStatics.CreateSaveGameObject` "/Game/Blueprints/Saves/BP_Save_Main.BP_Save_Main_C"))
      (bind _output_get (set `self.SaveMainRef` _returnvalue_3))
      (`GameplayStatics.SaveGameToSlot` _output_get (`self.SaveMainName`))))
  (bind _asbp_save_main (cast `/Game/Blueprints/Saves/BP_Save_Main` (`self.SaveMainRef`)))
  (`self.K2_SetActorLocation` (`/Game/Blueprints/Saves/BP_Save_Main.PlayerLocation` _asbp_save_main)))

(fn `SaveMain`
  (bind _returnvalue (`GameplayStatics.DoesSaveGameExist` (`self.SaveMainName`)))
  (if _returnvalue
    (bind _returnvalue_2 (`GameplayStatics.LoadGameFromSlot` (`self.SaveMainName`)))
    (set `self.SaveMainRef` _returnvalue_2)
    (else
      (bind _returnvalue_3 (`GameplayStatics.CreateSaveGameObject` "/Game/Blueprints/Saves/BP_Save_Main.BP_Save_Main_C"))
      (bind _output_get (set `self.SaveMainRef` _returnvalue_3))))
  (bind _asbp_save_main (cast `/Game/Blueprints/Saves/BP_Save_Main` _output_get))
  (set `/Game/Blueprints/Saves/BP_Save_Main.PlayerLocation` (`self.K2_GetActorLocation`) _asbp_save_main)
  (`GameplayStatics.SaveGameToSlot` (`self.SaveMainRef`) (`self.SaveMainName`)))

(fn `ShowInGameHUD`
  (`/Engine/EditorBlueprintResources/StandardMacros.IsValid` (`self.In-Game HUD`)
    (:`Is Valid`
      _)
    (:`Is Not Valid`
      (bind _returnvalue (`|CreateWidget` "/Game/Widgets/HUD/WBP_In-Game_HUD.WBP_In-Game_HUD_C" (`self.PlayerController`)))
      (bind _output_get (set `self.In-Game HUD` _returnvalue))))
  (`UserWidget.AddToViewport` _output_get 0)
  (return))

(fn `UserConstructionScript`)